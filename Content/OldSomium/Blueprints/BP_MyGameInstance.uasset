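; Game instance Blueprint that holds a global counter, relays Dode increments to the player and starts soundtrack playback.
; The Dode event increments the BP_Joueur count and refreshes its HUD state widget, then calls FaceReveal on a valid win widget or otherwise calls WinDode.
; PlayOST creates, stores and plays a 2D SC_OST sound with optional persistence across level transitions, leaving its Sound input unused.
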(event Custom|Count
  (Variables|Default|SetCountInt (+ (Variables|Default|GetCountInt) 1)))

(event Custom|GameInst%20Dode%20Incrementation
  (bind _returnvalue (Game|GetPlayerCharacter 0))
  (bind _asbp_joueur (Utilities|Casting|CastToBP_Joueur _returnvalue))
  (bind _wb_dodewin (Variables|/Game/OldSomium/Blueprints/GPE/BP_Joueur.BP_Joueur_C|GetWB_DodeWin _asbp_joueur))
  (Default|EventDodeIncrementation _asbp_joueur)
  (Default|UpdateEtatDodeUI (Variables|/Game/OldSomium/Blueprints/Ui/Crosshair/WBP_HUD1.WBP_HUD1_C|GetWB_EtatDode (Variables|/Game/OldSomium/Blueprints/GPE/BP_Joueur.BP_Joueur_C|GetMyHUD _asbp_joueur)))
  (Utilities|IsValid _wb_dodewin
    (:Is%20Valid
      (Default|FaceReveal _wb_dodewin))
    (:Is%20Not%20Valid
      (Default|WinDode _asbp_joueur))))

(fn PlayOST
  (params (Sound :type Sound%20Base%20Object%20Reference) (VolumeMultiplier :type Float%20%28single-precision%29) (bPersistAcrossLevelTransition? :type Boolean))
  (bind _returnvalue (Audio|CreateSound2D "/Game/FirstPerson/FX/SFX/OST/SC_OST.SC_OST" VolumeMultiplier 1.0 0.0 0 bPersistAcrossLevelTransition?))
  (bind _output_get (Variables|Default|SetAudio _returnvalue))
  (Audio|Components|Audio|Play _output_get 0.0))