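; BP_Light_Level_Air is a level light actor that fades its lights to the ColorWin color when the game instance signals an air light change.
; On BeginPlay it binds ColorSwitch to the ChangelightAir event on BP_MyGameInstance.
; ColorSwitch plays the Alpha timeline to recolor two point lights, via SwitchColor, and a rect light.
; Each update lerps from the light's current color, so the blend compounds rather than following the curve directly.
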(event Custom|ColorSwitch
  (bind _rectlight (Variables|Default|GetRectLight))
  (bind _alpha (Timeline|Alpha Play)
    (:Update
      (CallFunction|SwitchColor (Variables|Default|GetPointLight1) _alpha)
      (CallFunction|SwitchColor (Variables|Default|GetPointLight) _alpha)
      (Rendering|Components|Light|SetLightColor _rectlight (Math|Color|Lerp(LinearColor) (Rendering|Components|Light|GetLightColor _rectlight) (Math|Conversions|ToLinearColor(Color) (Variables|Default|GetColorWin)) _alpha) true))))

(event EventBeginPlay
  (bind _asbp_my_game_instance (Utilities|Casting|CastToBP_MyGameInstance (Game|GetGameInstance)))
  (EventDispatchers|BindEventtoChangelightAir _asbp_my_game_instance (delegate Custom|ColorSwitch)))

(event Collision|EventActorBeginOverlap
  (params (OtherActor :type Actor%20Object%20Reference)))

(event EventTick
  (params (DeltaSeconds :type Float%20%28single-precision%29)))

(fn ConstructionScript)

(fn SwitchColor
  (params (Light :type Point%20Light%20Component%20Object%20Reference) (Alpha :type Float%20%28double-precision%29))
  (Rendering|Components|Light|SetLightColor Light (Math|Color|Lerp(LinearColor) (Rendering|Components|Light|GetLightColor Light) (Math|Conversions|ToLinearColor(Color) (Variables|Default|GetColorWin)) Alpha) true)
  (return))