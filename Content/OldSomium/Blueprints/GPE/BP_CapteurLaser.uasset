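; BP_CapteurLaser is a sensor puzzle element that fires once on interaction, notifying its attached button and playing a sound.
; A room's final sensor then updates Game Instance progress, recolors the room by element through lights and timelines driving MPC_Color, and refreshes the player's dodecahedron HUD.
; The sensor-type switch for doors and teleport portals is disconnected, as is the old dodecahedron material and Niagara reveal logic.
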(event Custom|ChangeRoomColor
  (bind _as_bp_my_game_instance (Variables|Default|GetAs%20BP%20My%20Game%20Instance))
  (bind _as_bp_my_game_instance_2 (Variables|Default|GetAs%20BP%20My%20Game%20Instance))
  ;[1 1 1] Changement de couleur salle
  (switch Utilities|FlowControl|Switch|SwitchonENUM_RoomType (.roomtype (Variables|Default|GetStruct_Level&Room))
    (:NewEnumerator0
      (Default|CallChangelightFire _as_bp_my_game_instance_2)
      (bind _color_fire (Timeline|Color_room_fire Play)
        (:Update
          (Rendering|Material|SetVectorParameterValue "/Game/OldSomium/ART/Materials/MPC_Color.MPC_Color" "Color_room_fire" _color_fire :!class /Script/Engine.KismetMaterialLibrary))))
    (:NewEnumerator1
      (Default|CallChangelightAir _as_bp_my_game_instance_2)
      (bind _color_fire_2 (Timeline|Color_room_air Play)
        (:Update
          (Rendering|Material|SetVectorParameterValue "/Game/OldSomium/ART/Materials/MPC_Color.MPC_Color" "Color_room_air" _color_fire_2 :!class /Script/Engine.KismetMaterialLibrary))))
    (:NewEnumerator2
      (Default|CallChangelightEarth _as_bp_my_game_instance)
      (bind _color_fire_3 (Timeline|Color_room_earth Play)
        (:Update
          (Rendering|Material|SetVectorParameterValue "/Game/OldSomium/ART/Materials/MPC_Color.MPC_Color" "Color_room_earth" _color_fire_3 :!class /Script/Engine.KismetMaterialLibrary))))
    (:NewEnumerator3
      (Default|CallChangelightEther _as_bp_my_game_instance)
      (bind _color_fire_4 (Timeline|color_room_ether Play)
        (:Update
          (Rendering|Material|SetVectorParameterValue "/Game/OldSomium/ART/Materials/MPC_Color.MPC_Color" "Color_room_ether" _color_fire_4 :!class /Script/Engine.KismetMaterialLibrary))))
    (:NewEnumerator4
      (Default|CallChangelightWater _as_bp_my_game_instance)
      (bind _color_fire_5 (Timeline|Color_room_water Play)
        (:Update
          (Rendering|Material|SetVectorParameterValue "/Game/OldSomium/ART/Materials/MPC_Color.MPC_Color" "Color_room_water" _color_fire_5 :!class /Script/Engine.KismetMaterialLibrary))))))

(event EventBeginPlay
  (bind _asbp_my_game_instance (Utilities|Casting|CastToBP_MyGameInstance (Game|GetGameInstance)))
  (Variables|Default|SetAs%20BP%20My%20Game%20Instance _asbp_my_game_instance)
  (bind _asbp_joueur (Utilities|Casting|CastToBP_Joueur (Game|GetPlayerCharacter 0)))
  (Variables|Default|SetAs%20BP%20Joueur _asbp_joueur))

(event EventInteractionCapteur
  (bind _as_bp_my_game_instance (Variables|Default|GetAs%20BP%20My%20Game%20Instance))
  (Utilities|FlowControl|DoOnce false
    (:Completed
      (Class|BPInteraction|InteractionCapteur(Message) (Variables|Default|GetAttachedBoutons))
      (CallFunction|CapteurActivé)
      (Audio|PlaySoundatLocation 0 (Transformation|GetWorldLocation (Variables|Default|GetStaticMesh)) "0, 0, 0" 1.0 1.0 0.0 0 0 0 0)
      (if (Variables|Default|GetCapteurFinalSalle?)
        (Utilities|FlowControl|Delay 1.0)
        (Default|Count _as_bp_my_game_instance)
        (Default|GameInstDodeIncrementation _as_bp_my_game_instance)
        (CallFunction|ChangeRoomColor)
        (Default|UpdateEtatDodeUI (Variables|/Game/OldSomium/Blueprints/Ui/Crosshair/WBP_HUD1.WBP_HUD1_C|GetWB_EtatDode (Variables|/Game/OldSomium/Blueprints/GPE/BP_Joueur.BP_Joueur_C|GetMyHUD (Variables|Default|GetAs%20BP%20Joueur))))))))

(fn ConstructionScript)

(fn SwitchonCapteurType)

(fn CapteurActivé
  (CallFunction|SwitchonCapteurType))

(fn GetSpawnPortalLoc&Rot
  (bind _portalspawn (Variables|Default|GetPortalSpawn))
  (return (Transformation|GetWorldLocation _portalspawn) (Transformation|GetWorldRotation _portalspawn)))