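; BP_TutoDoor is a tutorial door with four sliding panels, opened either by player proximity or, in WorkWithLaser mode, by the InteractionCapteurTuto sensor event.
; One timeline plays and reverses the panel motion, with open and close sounds.
; On leaving the main trigger, a dot-product side test decides locking and, for laser doors, closing.
; A second trigger locks it and, after a delay, calls CallDoorShut on the player.
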(event OnComponentBeginOverlap(Box)
  (params (OverlappedComponent :type Primitive%20Component%20Object%20Reference) (OtherActor :type Actor%20Object%20Reference) (OtherComp :type Primitive%20Component%20Object%20Reference) (OtherBodyIndex :type Integer) (bFromSweep :type Boolean) (SweepResult :type Hit%20Result%20Structure%20%28by%20ref%29))
  ;[1 1 1] Si joueur entre TB porte, et si porte est entrée d'une salle et n'est pas lock, alors l'ouvrir
  (if (Actor|ActorHasTag OtherActor "Joueur")
    (if (not (Variables|Default|GetIs%20door%20locked))
      (if (not (Variables|Default|GetWorkWithLaser))
        (CallFunction|PlayDoorAnim)
        (Variables|Default|SetIsDoorClosed? false)))))

(event OnComponentEndOverlap(Box)
  (params (OverlappedComponent :type Primitive%20Component%20Object%20Reference) (OtherActor :type Actor%20Object%20Reference) (OtherComp :type Primitive%20Component%20Object%20Reference) (OtherBodyIndex :type Integer))
  ;[1 1 1] Joueur quitte TB de la porte : check si il faut fermer la porte et la locker, et le fait ou pas
  (if (Actor|ActorHasTag OtherActor "Joueur")
    (Variables|Default|SetDot%20Value (CallFunction|CheckifPlayerBehindorinFrontOfDoor))
    (if (not (Variables|Default|GetIs%20door%20locked))
      (if (Variables|Default|GetWorkWithLaser)
        ;;[1 1 1] Porte Fin de salle : Si joueur derrière la porte, la fermer, la lock
        (if (CallFunction|IsPlayerBehindDoor?)
          (CallFunction|AnimClosed)
          (Variables|Default|SetIsDoorClosed? true)
          (Variables|Default|SetIs%20door%20locked true))
        (else
          ;;[1 1 1] Porte d'entrée de salle : Fermer la porte et si il est derrière (dans la salle) la lock
          (CallFunction|AnimClosed)
          (Variables|Default|SetIsDoorClosed? true)
          (if (CallFunction|IsPlayerBehindDoor?)
            (Variables|Default|SetIs%20door%20locked true)))))))

(event OnComponentBeginOverlap(Box1)
  (params (OverlappedComponent :type Primitive%20Component%20Object%20Reference) (OtherActor :type Actor%20Object%20Reference) (OtherComp :type Primitive%20Component%20Object%20Reference) (OtherBodyIndex :type Integer) (bFromSweep :type Boolean) (SweepResult :type Hit%20Result%20Structure%20%28by%20ref%29))
  ;[1 1 1] Si joueur hit TB2 de la porte, alors locker la porte, et unload la salle précédente
  (if (Actor|ActorHasTag OtherActor "Joueur")
    (Variables|Default|SetIs%20door%20locked true)
    (Utilities|FlowControl|Delay 1.5)
    (Default|CallDoorShut! (Variables|Default|GetMyBP_Joueur))))

(event Custom|DoorMovementTimelineAnswer
  ;[1 0 0.007137] ?? Ancien mouv porte ?
  (Timeline|Timeline_0 Reverse))

(event Custom|DoorMouvementTimeline
  ;[1 0 0.007137] ?? Ancien mouv porte ?
  (Timeline|Timeline_0 Play))

(event Custom|PlayDoorAnim
  (bind _leftdoor (Variables|Default|GetLeftDoor))
  (bind _downdoor (Variables|Default|GetDownDoor))
  (bind _rightdoor (Variables|Default|GetRightDoor))
  (bind _topdoor (Variables|Default|GetTopDoor))
  (bind _leftdoor_2 (Variables|Default|GetLeftDoor))
  (bind _rightdoor_2 (Variables|Default|GetRightDoor))
  (bind _downdoor_2 (Variables|Default|GetDownDoor))
  (bind _topdoor_2 (Variables|Default|GetTopDoor))
  (bind _relativelocation (Variables|/Script/Engine.SceneComponent|GetRelativeLocation _leftdoor))
  (bind _relativelocation_2 (Variables|/Script/Engine.SceneComponent|GetRelativeLocation _rightdoor_2))
  (bind _relativelocation_3 (Variables|/Script/Engine.SceneComponent|GetRelativeLocation _rightdoor))
  (bind _relativelocation_4 (Variables|/Script/Engine.SceneComponent|GetRelativeLocation _downdoor))
  (bind _relativelocation_5 (Variables|/Script/Engine.SceneComponent|GetRelativeLocation _topdoor))
  (bind _relativelocation_6 (Variables|/Script/Engine.SceneComponent|GetRelativeLocation _leftdoor_2))
  (bind _relativelocation_7 (Variables|/Script/Engine.SceneComponent|GetRelativeLocation _downdoor_2))
  (bind _relativelocation_8 (Variables|/Script/Engine.SceneComponent|GetRelativeLocation _topdoor_2))
  (Utilities|FlowControl|Sequence
    (:then_0
      (Audio|PlaySound2D "/Game/FirstPerson/FX/SFX/Sound/Porte/SFX_Door_Open_idea-001_Cue.SFX_Door_Open_idea-001_Cue" 1.0 1.0 0.0 0 0))
    (:then_1
      (bind (_direction _bottomdoor _topdoor_3 _rightdoor_3 _leftdoor_3) (Timeline|DoorAnimation Play)
        (:Update
          (if (Variables|Default|GetIsDoorClosed?)
            (Utilities|FlowControl|Sequence
              (:then_0
                (Transformation|SetRelativeLocation _downdoor (Math|Vector|MakeVector (.x _relativelocation_4) (.y _relativelocation_4) (Math|Float|Lerp 0.0 (.z _relativelocation_4) _bottomdoor)) false false))
              (:then_1
                (Transformation|SetRelativeLocation _topdoor (Math|Vector|MakeVector (.x _relativelocation_5) (.y _relativelocation_5) (Math|Float|Lerp 0.0 (.z _relativelocation_5) _topdoor_3)) false false))
              (:then_2
                (Transformation|SetRelativeLocation _rightdoor_2 (Math|Vector|MakeVector (.x _relativelocation_2) (Math|Float|Lerp 0.0 (.y _relativelocation_2) _rightdoor_3) (.z _relativelocation_2)) false false))
              (:then_3
                (Transformation|SetRelativeLocation _leftdoor_2 (Math|Vector|MakeVector (.x _relativelocation_6) (Math|Float|Lerp 0.0 (.y _relativelocation_6) _leftdoor_3) (.z _relativelocation_6)) false false)))
            (else
              (Utilities|FlowControl|Sequence
                (:then_0
                  (Transformation|SetRelativeLocation _downdoor_2 (Math|Vector|MakeVector (.x _relativelocation_7) (.y _relativelocation_7) (Math|Float|Lerp (.z _relativelocation_7) (Variables|Default|GetBottomDoorPos) _bottomdoor)) false false))
                (:then_1
                  (Transformation|SetRelativeLocation _topdoor_2 (Math|Vector|MakeVector (.x _relativelocation_8) (.y _relativelocation_8) (Math|Float|Lerp (.z _relativelocation_8) (Variables|Default|GetTopDoorPos) _topdoor_3)) false false))
                (:then_2
                  (Transformation|SetRelativeLocation _rightdoor (Math|Vector|MakeVector (.x _relativelocation_3) (Math|Float|Lerp (.y _relativelocation_3) (Variables|Default|GetRightDoorPos) _rightdoor_3) (.z _relativelocation_3)) false false))
                (:then_3
                  (Transformation|SetRelativeLocation _leftdoor (Math|Vector|MakeVector (.x _relativelocation) (Math|Float|Lerp (.y _relativelocation) (Variables|Default|GetLeftDoorPos) _leftdoor_3) (.z _relativelocation)) false false))))))))))

(event Custom|AnimClosed
  (bind _leftdoor (Variables|Default|GetLeftDoor))
  (bind _downdoor (Variables|Default|GetDownDoor))
  (bind _rightdoor (Variables|Default|GetRightDoor))
  (bind _topdoor (Variables|Default|GetTopDoor))
  (bind _leftdoor_2 (Variables|Default|GetLeftDoor))
  (bind _rightdoor_2 (Variables|Default|GetRightDoor))
  (bind _downdoor_2 (Variables|Default|GetDownDoor))
  (bind _topdoor_2 (Variables|Default|GetTopDoor))
  (bind _relativelocation (Variables|/Script/Engine.SceneComponent|GetRelativeLocation _leftdoor))
  (bind _relativelocation_2 (Variables|/Script/Engine.SceneComponent|GetRelativeLocation _rightdoor_2))
  (bind _relativelocation_3 (Variables|/Script/Engine.SceneComponent|GetRelativeLocation _rightdoor))
  (bind _relativelocation_4 (Variables|/Script/Engine.SceneComponent|GetRelativeLocation _downdoor))
  (bind _relativelocation_5 (Variables|/Script/Engine.SceneComponent|GetRelativeLocation _topdoor))
  (bind _relativelocation_6 (Variables|/Script/Engine.SceneComponent|GetRelativeLocation _leftdoor_2))
  (bind _relativelocation_7 (Variables|/Script/Engine.SceneComponent|GetRelativeLocation _downdoor_2))
  (bind _relativelocation_8 (Variables|/Script/Engine.SceneComponent|GetRelativeLocation _topdoor_2))
  (Utilities|FlowControl|Sequence
    (:then_0
      (Audio|PlaySound2D "/Game/FirstPerson/FX/SFX/Sound/Porte/SFX_Door_Close_idea_-002_Cue.SFX_Door_Close_idea_-002_Cue" 1.0 1.0 0.0 0 0))
    (:then_1
      (bind (_direction _bottomdoor _topdoor_3 _rightdoor_3 _leftdoor_3) (Timeline|DoorAnimation Reverse)
        (:Update
          (if (Variables|Default|GetIsDoorClosed?)
            (Utilities|FlowControl|Sequence
              (:then_0
                (Transformation|SetRelativeLocation _downdoor (Math|Vector|MakeVector (.x _relativelocation_4) (.y _relativelocation_4) (Math|Float|Lerp 0.0 (.z _relativelocation_4) _bottomdoor)) false false))
              (:then_1
                (Transformation|SetRelativeLocation _topdoor (Math|Vector|MakeVector (.x _relativelocation_5) (.y _relativelocation_5) (Math|Float|Lerp 0.0 (.z _relativelocation_5) _topdoor_3)) false false))
              (:then_2
                (Transformation|SetRelativeLocation _rightdoor_2 (Math|Vector|MakeVector (.x _relativelocation_2) (Math|Float|Lerp 0.0 (.y _relativelocation_2) _rightdoor_3) (.z _relativelocation_2)) false false))
              (:then_3
                (Transformation|SetRelativeLocation _leftdoor_2 (Math|Vector|MakeVector (.x _relativelocation_6) (Math|Float|Lerp 0.0 (.y _relativelocation_6) _leftdoor_3) (.z _relativelocation_6)) false false)))
            (else
              (Utilities|FlowControl|Sequence
                (:then_0
                  (Transformation|SetRelativeLocation _downdoor_2 (Math|Vector|MakeVector (.x _relativelocation_7) (.y _relativelocation_7) (Math|Float|Lerp (.z _relativelocation_7) (Variables|Default|GetBottomDoorPos) _bottomdoor)) false false))
                (:then_1
                  (Transformation|SetRelativeLocation _topdoor_2 (Math|Vector|MakeVector (.x _relativelocation_8) (.y _relativelocation_8) (Math|Float|Lerp (.z _relativelocation_8) (Variables|Default|GetTopDoorPos) _topdoor_3)) false false))
                (:then_2
                  (Transformation|SetRelativeLocation _rightdoor (Math|Vector|MakeVector (.x _relativelocation_3) (Math|Float|Lerp (.y _relativelocation_3) (Variables|Default|GetRightDoorPos) _rightdoor_3) (.z _relativelocation_3)) false false))
                (:then_3
                  (Transformation|SetRelativeLocation _leftdoor (Math|Vector|MakeVector (.x _relativelocation) (Math|Float|Lerp (.y _relativelocation) (Variables|Default|GetLeftDoorPos) _leftdoor_3) (.z _relativelocation)) false false))))))))))

(event EventBeginPlay
  (CallFunction|SetPlayerReference))

(event EventInteractionCapteurTuto
  ;[1 1 1] Quand Capteur activé, Ouvrir porte
  (Variables|Default|SetIsDoorClosed? false)
  (CallFunction|PlayDoorAnim))

(fn ConstructionScript)

(fn MakeDoorTimeline
  (params (TimelineRef :type Float%20%28double-precision%29) (SplineInput :type Spline%20Component%20Object%20Reference) (DoorInput :type Scene%20Component%20Object%20Reference))
  (Transformation|SetWorldLocation DoorInput (Spline|GetLocationatDistanceAlongSpline SplineInput (* TimelineRef (Spline|GetSplineLength SplineInput)) "World") false false))

(fn SetPlateFormLoc&Rot
  (params (DoorInput :type Scene%20Component%20Object%20Reference) (SplineInput :type Spline%20Component%20Object%20Reference))
  (Transformation|SetWorldLocation DoorInput (Spline|GetLocationatDistanceAlongSpline SplineInput 0.0 "World") false false))

(fn IsPlayerBehindDoor?
  (return (>= (Variables|Default|GetDot%20Value) 0.0)))

(fn CheckifPlayerBehindorinFrontOfDoor
  (return (Math|Vector|DotProduct (Transformation|GetActorForwardVector) (Math|Vector|Normalize (- (Transformation|GetActorLocation) (Transformation|GetActorLocation (Variables|Default|GetMyBP_Joueur)))))))

(fn SetPlayerReference
  (bind _asbp_joueur (Utilities|Casting|CastToBP_Joueur (Game|GetPlayerCharacter 0)))
  (Variables|Default|SetMyBP_Joueur _asbp_joueur))