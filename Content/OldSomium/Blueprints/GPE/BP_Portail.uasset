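; BP_Portail is a level portal that sends the player to the main hub, Photonique or Plateformes level, chosen by EnumLevel.
; The construction script sets both portal meshes' materials to match that destination.
; On BeginPlay, the game instance's LevelCount decides whether a level portal is hidden, without changing its collision; the hub portal stays visible.
; Player overlap calls LOADING on BP_Joueur, waits briefly, then opens the destination map.
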(event OnComponentBeginOverlap(Portail)
  (params (OverlappedComponent :type Primitive%20Component%20Object%20Reference) (OtherActor :type Actor%20Object%20Reference) (OtherComp :type Primitive%20Component%20Object%20Reference) (OtherBodyIndex :type Integer) (bFromSweep :type Boolean) (SweepResult :type Hit%20Result%20Structure%20%28by%20ref%29))
  (bind _asbp_joueur (Utilities|Casting|CastToBP_Joueur OtherActor))
  (Utilities|IsValid _asbp_joueur
    (:Is%20Valid
      (Default|LOADING _asbp_joueur)
      (Utilities|FlowControl|Delay 1.3)
      (CallFunction|SwitchonPortalDestination))))

(event EventBeginPlay
  (Rendering|SetActorHiddenInGame false)
  (bind _asbp_my_game_instance (Utilities|Casting|CastToBP_MyGameInstance (Game|GetGameInstance)))
  (bind _output_get (Variables|Default|SetAs%20BP%20My%20Game%20Instance _asbp_my_game_instance))
  (CallFunction|ActivateDesactivatePortal (Variables|/Game/OldSomium/Blueprints/BP_MyGameInstance.BP_MyGameInstance_C|GetLevelCount _output_get)))

(fn ConstructionScript
  (switch Utilities|FlowControl|Switch|SwitchonEnum_Level (Variables|Default|GetEnum_Level)
    (:NewEnumerator0
      (Rendering|Material|SetMaterial (Variables|Default|GetPortail1) 0 "/Game/FirstPerson/FX/Portal/M_Portal_Exit.M_Portal_Exit")
      (Rendering|Material|SetMaterial (Variables|Default|GetPortail) 0 "/Game/FirstPerson/FX/Portal/M_Portal_Exit2.M_Portal_Exit2"))
    (:NewEnumerator1
      (Rendering|Material|SetMaterial (Variables|Default|GetPortail1) 0 "/Game/FirstPerson/FX/Portal/M_Portal_Level1_inst1.M_Portal_Level1_inst1")
      (Rendering|Material|SetMaterial (Variables|Default|GetPortail) 0 "/Game/FirstPerson/FX/Portal/M_Portal_Level1_inst2.M_Portal_Level1_inst2"))
    (:NewEnumerator2
      (Rendering|Material|SetMaterial (Variables|Default|GetPortail1) 0 "/Game/FirstPerson/FX/Portal/M_Portal_Level1_inst2_2.M_Portal_Level1_inst2_2")
      (Rendering|Material|SetMaterial (Variables|Default|GetPortail) 0 "/Game/FirstPerson/FX/Portal/M_Portal_Level2_inst2.M_Portal_Level2_inst2"))))

(fn SwitchonPortalDestination
  (switch Utilities|FlowControl|Switch|SwitchonEnum_Level (Variables|Default|GetEnum_Level)
    (:NewEnumerator0
      (Game|OpenLevel(byObjectReference) "/Game/FirstPerson/Maps/HUB-PH.HUB-PH"))
    (:NewEnumerator1
      (Game|OpenLevel(byObjectReference) "/Game/FirstPerson/Maps/Map_Photonique.Map_Photonique"))
    (:NewEnumerator2
      (Game|OpenLevel(byObjectReference) "/Game/FirstPerson/Maps/Map_2_Plateformes.Map_2_Plateformes"))))

(fn ActivateDesactivatePortal
  (params (LevelCount :type Integer))
  (Variables|Default|SetLevel%20Count LevelCount)
  (switch Utilities|FlowControl|Switch|SwitchonEnum_Level (Variables|Default|GetEnum_Level)
    (:NewEnumerator1
      (if (!= (Variables|Default|GetLevel%20Count) 0)
        (Rendering|SetActorHiddenInGame true)))
    (:NewEnumerator2
      (if (!= (Variables|Default|GetLevel%20Count) 1)
        (Rendering|SetActorHiddenInGame true)))))