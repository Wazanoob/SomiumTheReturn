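; AC_SoundWave is a GPE component that fires a sonic wave when activated through its parent's Act interface.
; Act runs the parent logic, then calls SpawnSoundWave, which spawns a BP_SonicWaveProjectile and an effect system at the given transform, with a sound attached to that effect.
; Deac only defers to the parent, and the component has no active BeginPlay or Tick logic.
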(event EventBeginPlay
  (|CallParentFunction) ; This node is disabled and will not be called.\nDrag off pins to build functionality.
)

(event EventTick
  (params (DeltaSeconds :type Float%20%28single-precision%29))
  (|CallParentFunction DeltaSeconds) ; This node is disabled and will not be called.\nDrag off pins to build functionality.
)

(fn Act
  (|CallParentFunction)
  (CallFunction|SpawnSoundWave))

(fn SpawnSoundWave
  (params (SpawnTransform :type Transform))
  (Game|SpawnActorfromClass "/Game/OldSomium/Blueprints/GPE/BP_SonicWaveProjectile.BP_SonicWaveProjectile_C" SpawnTransform "Undefined" 0 0)
  (bind _returnvalue (Niagara|SpawnSystematLocation 0 (.location SpawnTransform) (.rotation SpawnTransform) (.scale SpawnTransform)))
  (Audio|SpawnSoundAttached 0 _returnvalue "None" "0, 0, 0" "0, 0, 0" "KeepRelativeOffset" false 1.0 1.0 0.0 0 0))

(fn Deac
  (|CallParentFunction))