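; Interaction component that detects what the player looks at and triggers interactions with button actors.
; A looping timer sphere-traces from the camera manager, caches the hit actor and sends pointed start/end interface messages as focus is tracked.
; CheckForInteract runs a wider sphere trace from just below BP_Joueur's first-person camera, messaging hit actors tagged "Bouton" that implement BP_Interaction.
; Beam VFX and pause-time widget interaction nodes are disconnected.
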(event Custom|LineTraceInteraction
  (bind _returnvalue (Game|GetPlayerCameraManager 0))
  (bind _returnvalue_2 (Transformation|GetActorLocation _returnvalue))
  (bind _outhit (Collision|SphereTraceByChannel _returnvalue_2 (+ _returnvalue_2 (* (Transformation|GetActorForwardVector _returnvalue) (Variables|Default|GetTrace%20Distance))) 1e+01 "TraceTypeQuery1" false 0 "None"))
  (Utilities|IsValid (Variables|Default|GetHit%20Actor)
    (:Is%20Valid
      (if (!= (.HitActor (Collision|BreakHitResult _outhit)) (Variables|Default|GetHit%20Actor))
        (Class|BPInteraction|ObjectPointedEnd(Message) (Variables|Default|GetHit%20Actor))
        (Class|BPInteraction|ObjectPointedStart(Message) (Variables|Default|GetHit%20Actor))
        (Variables|Default|SetHit%20Actor (.HitActor (Collision|BreakHitResult _outhit)))
        (else
          (Class|BPInteraction|ObjectPointedStart(Message) (.HitActor (Collision|BreakHitResult _outhit)) :!label _label)
          (Variables|Default|SetHit%20Actor (.HitActor (Collision|BreakHitResult _outhit))))))
    (:Is%20Not%20Valid
      (goto _label))))

(event EventBeginPlay
  (bind _returnvalue (Utilities|Time|SetTimerbyEvent (delegate Custom|LineTraceInteraction) 0.3 true))
  (Variables|Default|SetTimerLineTraceInteraction _returnvalue))

(event EventTick
  (params (DeltaSeconds :type Float%20%28single-precision%29)))

(fn GetLineTrace
  (bind _returnvalue (Game|GetPlayerCharacter 0))
  (bind _asbp_joueur (Utilities|Casting|CastToBP_Joueur _returnvalue))
  (bind _firstpersoncamera (Variables|/Game/OldSomium/Blueprints/GPE/BP_Joueur.BP_Joueur_C|GetFirstPersonCamera _asbp_joueur))
  (bind _returnvalue_2 (Transformation|GetWorldLocation _firstpersoncamera))
  (bind _returnvalue_3 (- (.z _returnvalue_2) 18.0))
  (return (Math|Vector|MakeVector (.x _returnvalue_2) (.y _returnvalue_2) _returnvalue_3) (+ (Math|Vector|MakeVector (.x _returnvalue_2) (.y _returnvalue_2) _returnvalue_3) (* (Math|Vector|GetForwardVector (Transformation|GetWorldRotation _firstpersoncamera)) (Variables|Default|GetTrace%20Distance)))))

(fn CheckforInteract
  (bind (_starttrace _endtrace) (CallFunction|GetLineTrace))
  (bind _outhit (Collision|SphereTraceByChannel _starttrace _endtrace 5e+01 "TraceTypeQuery1" false 0 "None"))
  (if (.bBlockingHit (Collision|BreakHitResult _outhit))
    (if (and (Actor|ActorHasTag (.HitActor (Collision|BreakHitResult _outhit)) "Bouton") (Utilities|DoesObjectImplementInterface (.HitActor (Collision|BreakHitResult _outhit)) "/Game/OldSomium/Blueprints/GPE/BP_Interaction.BP_Interaction_C"))
      (Class|BPInteraction|InteractionJoueur(Message) (.HitActor (Collision|BreakHitResult _outhit))))))