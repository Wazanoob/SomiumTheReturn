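; AC_Laser is a laser component that fires a visible ray able to trigger prisms and sensors.
; ShootLaser spawns a red Niagara beam, line-traces on Visibility to set its endpoint, and adds smoke at any blocking impact.
; Prism hits receive a prism-laser message, other BP_Interaction actors get a sensor message, and SpawnLaserPrisme simply forwards to ShootLaser.
; Disconnected leftovers hold an abandoned sphere trace and a reflected second-ray trace.
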(fn ShootLaser
  (params (StartTrace :type Vector) (EndTrace :type Vector) (IsLaserLocked :type Boolean))
  ;[1 1 1] Premier Rayon.
  (bind _returnvalue (Niagara|SpawnSystematLocation "/Game/FirstPerson/FX/VFX/IES_Laser/NS_LaserRay.NS_LaserRay" StartTrace))
  (Effects|Components|ParticleSystem|SetColorParameter _returnvalue "Color" "(R=0.557292,G=0.055370,B=0.022086,A=1.000000)")
  (bind (_outhit _returnvalue_2) (Collision|LineTraceByChannel StartTrace EndTrace "TraceTypeQuery1" false 0 "None"))
  (Effects|Components|ParticleSystem|SetVectorParameter _returnvalue "LaserEnd" (select (.bBlockingHit (Collision|BreakHitResult _outhit)) (.ImpactPoint (Collision|BreakHitResult _outhit)) EndTrace))
  (if (.bBlockingHit (Collision|BreakHitResult _outhit))
    (Niagara|SpawnSystematLocation "/Game/FirstPerson/FX/VFX/IES/IES_Niagara/NS/NS_Smokes.NS_Smokes" (.ImpactPoint (Collision|BreakHitResult _outhit))))
  (if (Utilities|DoesObjectImplementInterface (.HitActor (Collision|BreakHitResult _outhit)) "/Game/OldSomium/Blueprints/GPE/BP_Interaction.BP_Interaction_C")
    (if (== (.HitActor (Collision|BreakHitResult _outhit)) "/Game/OldSomium/Blueprints/GPE/BP_Prisme.BP_Prisme_C")
      (if (and _returnvalue_2 (== (.HitActor (Collision|BreakHitResult _outhit)) "/Game/OldSomium/Blueprints/GPE/BP_Prisme.BP_Prisme_C")) :!label _label
        (Class|BPInteraction|InteractionPrismeLaser(Message) (.HitActor (Collision|BreakHitResult _outhit))))
      (else
        (Class|BPInteraction|InteractionCapteur(Message) (.HitActor (Collision|BreakHitResult _outhit)))))
    (else
      (goto _label))))

(fn SpawnLaserPrisme
  (params (StartTrace :type Vector) (EndTrace :type Vector) (IsLaserLocked? :type Boolean))
  (CallFunction|ShootLaser StartTrace EndTrace IsLaserLocked?))