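; AC_P_Tools is an actor component that appears to serve as a base for player tools.
; Act and Deac are empty stubs, and the event graph has no active logic.
; GetLineTrace supplies trace endpoints without tracing: it starts at the BP_Joueur player's Dodecahedron and extends TraceDistance along the first-person camera's forward vector.
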(event EventBeginPlay)

(event EventTick
  (params (DeltaSeconds :type Float%20%28single-precision%29)))

(fn Act)

(fn Deac)

(fn GetLineTrace
  (bind _returnvalue (Game|GetPlayerCharacter 0))
  (bind _asbp_joueur (Utilities|Casting|CastToBP_Joueur _returnvalue))
  (bind _dodecahedron (Variables|/Game/OldSomium/Blueprints/GPE/BP_Joueur.BP_Joueur_C|GetDodecahedron _asbp_joueur))
  (bind _returnvalue_2 (Transformation|GetWorldLocation _dodecahedron))
  (return _returnvalue_2 (+ _returnvalue_2 (* (Math|Vector|GetForwardVector (Transformation|GetWorldRotation (Variables|/Game/OldSomium/Blueprints/GPE/BP_Joueur.BP_Joueur_C|GetFirstPersonCamera _asbp_joueur))) (LocalVariables|GetTraceDistance)))))