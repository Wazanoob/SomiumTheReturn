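; Silice gun target zone, from an old GPE version, that relays silice projectile impacts to a linked button (BoutonLié).
; On Hit, it casts the other actor to BP_SiliceProjectile and, if valid, calls InteractionSiliceMessage on that button.
; BeginPlay and the construction script also send this message, with both branches of the Activated check making the same call.
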(event EventBeginPlay
  (bind _boutonlié (Variables|Default|GetBoutonLié))
  (if (Variables|Default|GetActivated?)
    (Class|BPInteraction|InteractionSilice(Message) _boutonlié)
    (else
      (Class|BPInteraction|InteractionSilice(Message) _boutonlié))))

(event Collision|EventHit
  (params (MyComp :type Primitive%20Component%20Object%20Reference) (Other :type Actor%20Object%20Reference) (OtherComp :type Primitive%20Component%20Object%20Reference) (bSelfMoved :type Boolean) (HitLocation :type Vector :default "0, 0, 0") (HitNormal :type Vector :default "0, 0, 0") (NormalImpulse :type Vector :default "0, 0, 0") (Hit :type Hit%20Result%20Structure%20%28by%20ref%29))
  ;[1 1 1] Lors de la collision avec la silice
  (Utilities|IsValid (.AsBP%20Silice%20Projectile (Utilities|Casting|CastToBP_SiliceProjectile Other))
    (:Is%20Valid
      (Class|BPInteraction|InteractionSilice(Message) (Variables|Default|GetBoutonLié)))))

(fn ConstructionScript
  (bind _boutonlié (Variables|Default|GetBoutonLié))
  (if (Variables|Default|GetActivated?)
    (Class|BPInteraction|InteractionSilice(Message) _boutonlié)
    (else
      (Class|BPInteraction|InteractionSilice(Message) _boutonlié))))