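; BP_Hub is an interactable hub that triggers its linked buttons (BoutonsLiés) on player interaction.
; A sphere overlap tracks whether BP_Joueur is in range and swaps the mesh material between gold and red.
; InteractionJoueur, when in range, spawns an explosion at the cylinder and sends InteractionHubMessage to the linked actors.
; On overlap, temporary debug spheres mark up to three linked buttons using a height-offset location helper.
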(event OnComponentBeginOverlap(Sphere)
  (params (OverlappedComponent :type Primitive%20Component%20Object%20Reference) (OtherActor :type Actor%20Object%20Reference) (OtherComp :type Primitive%20Component%20Object%20Reference) (OtherBodyIndex :type Integer) (bFromSweep :type Boolean) (SweepResult :type Hit%20Result%20Structure%20%28by%20ref%29))
  (bind (_return_value_x _return_value_y _return_value_z _boutonsliés) (CallFunction|GetAttachedActorLocation+ZOFFSET 0 35.0))
  (bind (_return_value_x_2 _return_value_y_2 _return_value_z_2 _boutonsliés_2) (CallFunction|GetAttachedActorLocation+ZOFFSET 1 35.0))
  (bind (_return_value_x_3 _return_value_y_3 _return_value_z_3 _boutonsliés_3) (CallFunction|GetAttachedActorLocation+ZOFFSET 2 35.0))
  ;[1 1 1] EventInteractionJoueur
  (Utilities|IsValid (.AsBP%20Joueur (Utilities|Casting|CastToBP_Joueur OtherActor))
    (:Is%20Valid
      (Variables|Default|SetJoueurInRadius true)
      (Rendering|Material|SetMaterial (Variables|Default|GetStaticMesh1) 0 "/Game/FirstPerson/LevelPrototyping/Materials/PH_Mat_Room2_Playtest/MAT_Room2_Gold_Instance.MAT_Room2_Gold_Instance")
      ;[0.7823 0.11 0.11] DEBUG (DIRTY)
      (Utilities|FlowControl|Sequence
        (:then_0
          (Utilities|IsValid _boutonsliés
            (:Is%20Valid
              (Rendering|Debug|DrawDebugSphere (Math|Vector|MakeVector _return_value_x _return_value_y _return_value_z) 3e+01 12 "(R=0.000000,G=1.000000,B=0.036101,A=1.000000)" 2.0))))
        (:then_1
          (Utilities|IsValid _boutonsliés_2
            (:Is%20Valid
              (Rendering|Debug|DrawDebugSphere (Math|Vector|MakeVector _return_value_x_2 _return_value_y_2 _return_value_z_2) 3e+01 12 "(R=0.000000,G=1.000000,B=0.008980,A=1.000000)" 2.0))))
        (:then_2
          (Utilities|IsValid _boutonsliés_3
            (:Is%20Valid
              (Rendering|Debug|DrawDebugSphere (Math|Vector|MakeVector _return_value_x_3 _return_value_y_3 _return_value_z_3) 3e+01 12 "(R=0.000000,G=1.000000,B=0.069125,A=1.000000)" 2.0))))))))

(event OnComponentEndOverlap(Sphere)
  (params (OverlappedComponent :type Primitive%20Component%20Object%20Reference) (OtherActor :type Actor%20Object%20Reference) (OtherComp :type Primitive%20Component%20Object%20Reference) (OtherBodyIndex :type Integer))
  ;[1 1 1] EventInteractionJoueur
  (Utilities|IsValid (.AsBP%20Joueur (Utilities|Casting|CastToBP_Joueur OtherActor))
    (:Is%20Valid
      (Variables|Default|SetJoueurInRadius false)
      (Rendering|Material|SetMaterial (Variables|Default|GetStaticMesh1) 0 "/Game/OldSomium/ART/Materials/Couleurs/M_Red.M_Red"))))

(event EventInteractionJoueur
  ;[1 1 1] EventInteractionJoueur
  (if (Variables|Default|GetJoueurInRadius)
    (Effects|SpawnEmitteratLocation "/Game/UnrealContent/StarterContent/Particles/P_Explosion.P_Explosion" (Transformation|GetWorldLocation (Variables|Default|GetCylinder)))
    (Class|BPInteraction|InteractionHub(Message) (Variables|Default|GetBoutonsLiés))))

(fn ConstructionScript)

(fn GetAttachedActorLocation+ZOFFSET
  (params (IndexBouton :type Integer) (ZOffset :type Float%20%28double-precision%29))
  (bind _boutonsliés (Variables|Default|GetBoutonsLiés))
  (bind _output (Utilities|Array|Get(acopy) _boutonsliés IndexBouton))
  (bind _returnvalue (Transformation|GetActorLocation _output))
  (Utilities|IsValid _output
    (:Is%20Valid
      (return (.x _returnvalue) (.y _returnvalue) (+ (.z _returnvalue) ZOffset) _output))))