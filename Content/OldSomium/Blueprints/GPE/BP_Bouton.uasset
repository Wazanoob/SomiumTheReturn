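; BP_Bouton is a puzzle button that triggers its linked prism, with a prism or cannon mesh chosen at construction.
; Player presses, unless disabled by a sensor, or hub interactions, when a silice-toggled connection is active, message the prism with sound, rumble and a StopSign broadcast.
; Pointing at it sets custom-depth stencil, notifies the prism and shows a timeline-animated gamepad or keyboard prompt until StopSign is set.
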(event Custom|OverlapTrigger
  (params (MyPlane :type Static%20Mesh%20Component%20Object%20Reference))
  (bind _start_location (Variables|Default|GetStart%20Location))
  ;[1 1 1] UI début Overlap
  (Utilities|FlowControl|DoOnce false :!label _label
    (:Completed
      (bind _newtrack_0 (Timeline|MovementSign Play)
        (:Update
          (Transformation|SetRelativeLocation MyPlane (Math|Vector|Lerp(Vector) _start_location (+ _start_location (Variables|Default|GetEndLocation)) _newtrack_0) false false)
          (Utilities|FlowControl|Sequence
            (:then_0
              (Utilities|FlowControl|DoOnce false))
            (:then_1
              (goto _label Reset))))
        (:Finished
          (Utilities|FlowControl|Sequence
            (:then_0
              (Utilities|FlowControl|DoOnce false :!label _label_2
                (:Completed
                  (Timeline|MovementSign PlayFromStart))))
            (:then_1
              (goto _label_2 Reset))))))))

(event Custom|GPStopSign!
  (Variables|Default|SetStopSign! true))

(event Custom|KBStopSign!
  (Variables|Default|SetStopSign! true))

(event EventInteractionSilice
  (bind _props_gpe_boutonprism_object017 (Variables|Default|GetPROPS_GPE_Boutonprism_Object017))
  ;[1 0 0] SILICE
  (Utilities|FlowControl|FlipFlop
    (:A
      (Variables|Default|SetHubConnectionActive? true)
      (Rendering|Material|SetMaterial _props_gpe_boutonprism_object017 0 "/Game/OldSomium/ART/Materials/Couleurs/M_Green.M_Green"))
    (:B
      (Variables|Default|SetHubConnectionActive? false)
      (Rendering|Material|SetMaterial _props_gpe_boutonprism_object017 0 "/Game/OldSomium/ART/Materials/Couleurs/M_Purple.M_Purple"))))

(event EventInteractionJoueur
  ;[1 1 1] EventInteractionJoueur
  (if (Variables|Default|GetCanPlayerPush?)
    (Class|BPInteraction|InteractionBouton(Message) (Variables|Default|GetPrismeLié))
    (Rendering|Material|SetMaterial (Variables|Default|GetPROPS_GPE_Boutonprism_Object017) 0 "/Game/OldSomium/ART/Texture/Bouton/M_BoutonPrisme.M_BoutonPrisme")
    (Audio|SpawnSoundAttached "/Game/FirstPerson/FX/SFX/Sound/Prisme_et_Button/SC_Prisme_Button_01.SC_Prisme_Button_01" (Variables|Default|GetPROPS_GPE_Boutonprism_Object017) "None" "0, 0, 0" "0, 0, 0" "KeepRelativeOffset" false 1.0 1.0 0.0 0 0)
    (Default|CallStopSign)
    (Game|Feedback|PlayDynamicForceFeedback (Game|GetPlayerController 0) 0.1 1.0 true true true true)
    (else
      (Rendering|Material|SetMaterial (Variables|Default|GetPROPS_GPE_Boutonprism_Object017) 0 "/Game/OldSomium/ART/Materials/Environement/Master/M_Black_pipe.M_Black_pipe"))))

(event EventObjectPointedEnd
  (bind _props_gpe_boutonprism_object017 (Variables|Default|GetPROPS_GPE_Boutonprism_Object017))
  ;[1 1 1] Pointé par le joueur EVENT START/END
  (Utilities|FlowControl|Delay 0.0005)
  (Utilities|IsValid _props_gpe_boutonprism_object017
    (:Is%20Valid
      (Rendering|SetCustomDepthStencilValue _props_gpe_boutonprism_object017 0)
      (Class|BPInteraction|PrismePointedEnd(Message) (Variables|Default|GetPrismeLié)))))

(event EventInteractionHub
  ;[1 1 1] EventInteractionJoueur
  ;;[1 0 0] HUB
  (if (Variables|Default|GetHubConnectionActive?)
    (Class|BPInteraction|InteractionBouton(Message) (Variables|Default|GetPrismeLié))
    (Rendering|Material|SetMaterial (Variables|Default|GetPROPS_GPE_Boutonprism_Object017) 0 "/Game/OldSomium/ART/Texture/Bouton/M_BoutonPrisme.M_BoutonPrisme")
    (Audio|SpawnSoundAttached "/Game/FirstPerson/FX/SFX/Sound/Prisme_et_Button/SC_Prisme_Button_01.SC_Prisme_Button_01" (Variables|Default|GetPROPS_GPE_Boutonprism_Object017) "None" "0, 0, 0" "0, 0, 0" "KeepRelativeOffset" false 1.0 1.0 0.0 0 0)
    (Default|CallStopSign)
    (Game|Feedback|PlayDynamicForceFeedback (Game|GetPlayerController 0) 0.1 1.0 true true true true)))

(event EventBeginPlay
  ;[1 1 1] BEGIN PLAY
  (bind _asbp_joueur (Utilities|Casting|CastToBP_Joueur (Game|GetPlayerCharacter 0)))
  (bind _output_get (Variables|Default|SetAs%20BP%20Joueur _asbp_joueur))
  (if (Variables|/Game/OldSomium/Blueprints/GPE/BP_Joueur.BP_Joueur_C|GetIsUsingGamepad _output_get)
    (Variables|Default|SetStart%20Location (Variables|/Script/Engine.SceneComponent|GetRelativeLocation (Variables|Default|GetGP_Plane)))
    (else
      (Variables|Default|SetStart%20Location (Variables|/Script/Engine.SceneComponent|GetRelativeLocation (Variables|Default|GetKB_Plane))))))

(event EventInteractionCapteur
  (Variables|Default|SetCanPlayerPush? false))

(event EventObjectPointedStart
  (bind _kb_plane (Variables|Default|GetKB_Plane))
  (bind _gp_plane (Variables|Default|GetGP_Plane))
  (bind _stopsign_ (Variables|Default|GetStopSign!))
  (bind _props_gpe_boutonprism_object017 (Variables|Default|GetPROPS_GPE_Boutonprism_Object017))
  ;[1 1 1] Pointé par le joueur EVENT START/END
  (Utilities|IsValid _props_gpe_boutonprism_object017
    (:Is%20Valid
      (Rendering|SetCustomDepthStencilValue _props_gpe_boutonprism_object017 1)
      (Class|BPInteraction|PrismePointedStart(Message) (Variables|Default|GetPrismeLié))
      (if (Variables|/Game/OldSomium/Blueprints/GPE/BP_Joueur.BP_Joueur_C|GetIsUsingGamepad (Variables|Default|GetAs%20BP%20Joueur))
        (EventDispatchers|BindEventtoStopSign (delegate Custom|GPStopSign!))
        (if _stopsign_
          (Rendering|SetVisibility _gp_plane false false)
          (else
            (Rendering|SetVisibility _kb_plane false false)
            (Rendering|SetVisibility _gp_plane true false)
            (CallFunction|OverlapTrigger _gp_plane)))
        (else
          (EventDispatchers|BindEventtoStopSign (delegate Custom|KBStopSign!))
          (if _stopsign_
            (Rendering|SetVisibility _kb_plane false false)
            (else
              (Rendering|SetVisibility _gp_plane false false)
              (Rendering|SetVisibility _kb_plane true false)
              (CallFunction|OverlapTrigger _kb_plane))))))))

(fn ConstructionScript
  (bind _props_gpe_boutonprism_object017 (Variables|Default|GetPROPS_GPE_Boutonprism_Object017))
  (if (Variables|Default|GetConnectedToLaserPrism?)
    (Components|StaticMesh|SetStaticMesh (Variables|Default|GetPROPS_GPE_Boutonprism_Object017) "/Game/OldSomium/ART/Meshes/GPE/Panneau_commande/double/PROPS_GPE_CommandeDouble_prismbutton_push.PROPS_GPE_CommandeDouble_prismbutton_push")
    (else
      (Components|StaticMesh|SetStaticMesh (Variables|Default|GetPROPS_GPE_Boutonprism_Object017) "/Game/OldSomium/ART/Meshes/GPE/Panneau_commande/double/PROPS_GPE_CommandeDouble_canonbutton_push.PROPS_GPE_CommandeDouble_canonbutton_push")))
  (if (Variables|Default|GetHubConnectionActive?)
    (Rendering|Material|SetMaterial _props_gpe_boutonprism_object017 0 "/Game/OldSomium/ART/Texture/Bouton/M_BoutonPrisme.M_BoutonPrisme")
    (else
      (Rendering|Material|SetMaterial _props_gpe_boutonprism_object017 0 "/Game/OldSomium/ART/Texture/Bouton/M_BoutonPrisme.M_BoutonPrisme")))
  (CallFunction|SwitchonPrismState))

(fn SwitchonPrismState)