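; Rotatable puzzle prism that emits either a laser or sound waves, with construction script setting its mesh from IsLaser and IsSource.
; Button interaction advances a state enum (three directions for laser, four for sound) and a timeline rotates prism and tooltip.
; The state picks the spawn point passed to the laser or soundwave component.
; Interaction events trigger emission, while sources repeat it on looping timers, with lasers starting at BeginPlay.
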(event Custom|PrismMovementTimelineAnswer
  ;[1 0 0] PrismeRotationEvent
  (bind _traveldistance (Timeline|PrismRotation Reverse)
    (:Update
      (Transformation|SetRelativeRotation (Variables|Default|GetPrism) (Math|Rotator|MakeRotator 0.0 0.0 (* _traveldistance (.yaw (Math|Conversions|RotationFromXVector (Math|Vector|GetForwardVector (Variables|Default|GetSpawnLaserPoint0)))))) false false))
    (:Finished
      (Utilities|FlowControl|Delay 0.2))))

(event Custom|PrismMouvementTimeline
  ;[1 0 0] PrismeRotationEvent
  (bind _traveldistance (Timeline|PrismRotation Play)
    (:Update
      (Transformation|SetRelativeRotation (Variables|Default|GetPrism) (Math|Rotator|MakeRotator 0.0 0.0 (* _traveldistance (.yaw (Math|Conversions|RotationFromXVector (Math|Vector|GetForwardVector (Variables|Default|GetSpawnLaserPoint0)))))) false false))
    (:Finished
      (Utilities|FlowControl|Delay 0.2))))

(event Custom|LaserSpawnEvent
  ;[1 1 1] Définition de la localisation du spawn à partir de la fonction get line traces puis appel fonction spawn Laser Prisme du Laser Component
  (Utilities|FlowControl|DoOnce false :!label _label
    (:Completed
      (CallFunction|SpawnLaser)
      (if (Variables|Default|GetisSource?)
        (bind _returnvalue (Utilities|Time|SetTimerbyEvent (delegate Custom|LaserSpawnEvent) 0.1 true))
        (Variables|Default|SetLaserTimer _returnvalue)
        (goto _label Reset)
        (else
          (goto _label Reset))))))

(event Custom|TimelineRotEvent
  ;[1 1 1] TimelineRotation
  (Audio|SpawnSoundAttached 0 (Variables|Default|GetPrism) "None" "0, 0, 0" "0, 0, 0" "KeepRelativeOffset" false 1.0 1.0 0.0 0 0)
  (Utilities|FlowControl|DoOnce false :!label _label
    (:Completed
      (bind _rotation (Timeline|RotTimeline PlayFromStart)
        (:Update
          (switch Utilities|FlowControl|Switch|SwitchonENUM_PrismState (Variables|Default|GetENUM_PrismState)
            (:NewEnumerator1
              (Transformation|SetRelativeRotation (Variables|Default|GetPrism) (Math|Rotator|Lerp(Rotator) "0, 0, 0" "0.000000,-90.000000,0.000000" _rotation) false false))
            (:NewEnumerator2
              (Transformation|SetRelativeRotation (Variables|Default|GetPrism) (Math|Rotator|Lerp(Rotator) "0.000000,-90.000000, 0" "0.000000,-180.000000,0.000000" _rotation) false false))
            (:NewEnumerator3
              (Transformation|SetRelativeRotation (Variables|Default|GetPrism) (Math|Rotator|Lerp(Rotator) "0,-180.000000, 0" "0.000000,-270.000000,0.000000" _rotation true) false false))
            (:NewEnumerator4
              (Transformation|SetRelativeRotation (Variables|Default|GetPrism) (Math|Rotator|Lerp(Rotator) "0,-270.000000, 0" "0.000000,-360.000000,0.000000" _rotation true) false false))))
        (:Finished
          (goto _label Reset))))))

(event Custom|SoundWaveSpawnEvent
  ;[1 1 1] SpawnSoundWave Event
  (Utilities|FlowControl|DoOnce false :!label _label
    (:Completed
      (CallFunction|SpawnSoundWave)
      (if (Variables|Default|GetisSource?)
        (bind _returnvalue (Utilities|Time|SetTimerbyEvent (delegate Custom|SoundWaveSpawnEvent) 0.2 true))
        (Variables|Default|SetShockwaveTimerHandle _returnvalue)
        (goto _label Reset)
        (else
          (goto _label Reset))))))

(event EventInteractionPrismeLaser
  (bind _prism (Variables|Default|GetPrism))
  (bind _returnvalue (Transformation|GetWorldLocation _prism))
  ;[1 1 1] Lors de l'interaction du prisme avec le laser
  (if (Variables|Default|GetisLaser?)
    (CallFunction|LaserSpawnEvent)
    (else
      (Utilities|FlowControl|DoOnce false :!label _label
        (:Completed
          (Niagara|SpawnSystematLocation 0 (Math|Vector|MakeVector (.x _returnvalue) (.y _returnvalue) (+ (.z _returnvalue) 23.0)))
          (CallFunction|SoundWaveSpawnEvent)
          (Utilities|FlowControl|Delay 2.0)
          (goto _label Reset))))))

(event EventInteractionBouton
  ;[1 1 1] Interaction bouton
  (CallFunction|SwitchonSpawnPointEvent)
  (CallFunction|SwitchMatonPrismToolTip)
  (CallFunction|TimelineRotEvent))

(event EventBeginPlay
  ;[1 1 1] Lors de l'interaction du prisme avec le laser
  (Utilities|FlowControl|Sequence
    (:then_0
      (Variables|Default|SetStartRot (Variables|/Script/Engine.SceneComponent|GetRelativeRotation (Variables|Default|GetPrism))))
    (:then_1
      (if (Variables|Default|GetisSource?)
        (CallFunction|LaserSpawnEvent)))
    (:then_2
      (Audio|SpawnSoundAttached 0 (Variables|Default|GetPrism) "None" "0, 0, 0" "0, 0, 0" "KeepRelativeOffset" false 1.0 1.0 0.0 0 0))))

(event EventPrismePointedEnd
  ;[1 1 1] Illuminer Prisme
  (Rendering|SetCustomDepthStencilValue (Variables|Default|GetPrism) 0))

(event EventPrismePointedStart
  ;[1 1 1] Illuminer Prisme
  (Rendering|SetCustomDepthStencilValue (Variables|Default|GetPrism) 1))

(fn ConstructionScript
  (bind _prism (Variables|Default|GetPrism))
  (bind _prism_2 (Variables|Default|GetPrism))
  (bind _spawnlaserpoint1 (Variables|Default|GetSpawnLaserPoint1))
  (bind _spawnlaserpoint0 (Variables|Default|GetSpawnLaserPoint0))
  (CallFunction|SetSpawnPointsRelativeHeight)
  (CallFunction|SwitchMatonPrismToolTip)
  (CallFunction|SetPrismRelativeRotation)
  (if (Variables|Default|GetisLaser?)
    (Components|StaticMesh|SetStaticMesh (Variables|Default|GetTooltip) "/Game/OldSomium/ART/Meshes/GPE/Panneau_commande/double/PROPS_GPE_CommandeDouble_miniTriangle.PROPS_GPE_CommandeDouble_miniTriangle")
    (if (Variables|Default|GetisSource?)
      (Components|StaticMesh|SetStaticMesh (Variables|Default|GetPrism) "/Game/OldSomium/ART/Meshes/GPE/Prisme/PROPS_GPE_Source.PROPS_GPE_Source")
      (else
        (Components|StaticMesh|SetStaticMesh (Variables|Default|GetPrism) "/Game/OldSomium/ART/Meshes/GPE/Prisme/PROPS_GPE_Prism__3_.PROPS_GPE_Prism__3_")))
    (else
      (Components|StaticMesh|SetStaticMesh (Variables|Default|GetTooltip) "/Game/OldSomium/ART/Meshes/GPE/Panneau_commande/double/PROPS_GPE_CommandeDouble_miniCarré.PROPS_GPE_CommandeDouble_miniCarré")
      (Components|StaticMesh|SetStaticMesh (Variables|Default|GetPrism) "/Game/OldSomium/ART/Meshes/GPE/Prisme/PROPS_GPE_Bombox.PROPS_GPE_Bombox")))
  (if (Variables|Default|GetTrueLaserSpawnPointVisibleFromStart?)
    (switch Utilities|FlowControl|Switch|SwitchonENUM_PrismState (Variables|Default|GetENUM_PrismState)
      (:NewEnumerator1
        (Rendering|Material|SetMaterial _prism_2 5 "/Game/OldSomium/ART/Materials/Couleurs/M_Green.M_Green")
        (Rendering|Material|SetMaterial _prism_2 4 "/Game/OldSomium/ART/Materials/Couleurs/M_Red.M_Red")
        (Rendering|SetVisibility _spawnlaserpoint0 true false)
        (Rendering|SetVisibility _spawnlaserpoint1 false false))
      (:NewEnumerator2
        (Rendering|Material|SetMaterial _prism 5 "/Game/OldSomium/ART/Materials/Couleurs/M_Red.M_Red")
        (Rendering|Material|SetMaterial _prism 4 "/Game/OldSomium/ART/Materials/Couleurs/M_Green.M_Green")
        (Rendering|SetVisibility _spawnlaserpoint0 false false)
        (Rendering|SetVisibility _spawnlaserpoint1 true false))
      (:NewEnumerator3
        (Rendering|SetVisibility (Variables|Default|GetSpawnLaserPoint1) false false)
        (Rendering|SetVisibility (Variables|Default|GetSpawnLaserPoint2) true false))))
  (if (Variables|Default|GetSpawnPointVisible%28EDITOR%29)
    (Rendering|SetVisibility (Variables|Default|GetSpawnLaserPoint2) true false)
    (else
      (Rendering|SetVisibility (Variables|Default|GetSpawnLaserPoint2) false false))))

(fn GetLineTracesSpawnLocation
  (bind _spawnlaserpoint1 (Variables|Default|GetSpawnLaserPoint1))
  (bind _spawnlaserpoint0 (Variables|Default|GetSpawnLaserPoint0))
  (bind _spawnlaserpoint2 (Variables|Default|GetSpawnLaserPoint2))
  (bind _returnvalue (Transformation|GetWorldLocation _spawnlaserpoint0))
  (bind _returnvalue_2 (Transformation|GetWorldLocation _spawnlaserpoint1))
  (bind _returnvalue_3 (Transformation|GetWorldLocation _spawnlaserpoint2))
  (return (+ _returnvalue "0,0,8.400000") (+ _returnvalue (* (Math|Vector|GetForwardVector (Transformation|GetWorldRotation _spawnlaserpoint0)) (Variables|Default|GetLaserLength))) (+ _returnvalue_2 "0,0,8.400000") (+ _returnvalue_2 (* (Math|Vector|GetForwardVector (Transformation|GetWorldRotation _spawnlaserpoint1)) (Variables|Default|GetLaserLength))) (+ _returnvalue_3 "0,0,8.400000") (+ _returnvalue_3 (* (Math|Vector|GetForwardVector (Transformation|GetWorldRotation _spawnlaserpoint2)) (Variables|Default|GetLaserLength))) "0, 0, 0" "0, 0, 0"))

(fn SwitchonSpawnPointEvent
  (if (Variables|Default|GetisLaser?)
    (Audio|SpawnSoundAttached 0 (Variables|Default|GetPrism) "None" "0, 0, 0" "0, 0, 0" "KeepRelativeOffset" false 1.0 1.0 0.0 0 0))
  (switch Utilities|FlowControl|Switch|SwitchonENUM_PrismState (Variables|Default|GetENUM_PrismState)
    (:NewEnumerator1
      (Variables|Default|SetENUM_PrismState "NewEnumerator2"))
    (:NewEnumerator2
      (Variables|Default|SetENUM_PrismState "NewEnumerator3"))
    (:NewEnumerator3
      (if (Variables|Default|GetisLaser?)
        (Variables|Default|SetENUM_PrismState "NewEnumerator1" :!label _label)
        (else
          (Variables|Default|SetENUM_PrismState "NewEnumerator4"))))
    (:NewEnumerator4
      (goto _label))))

(fn SpawnLaser
  (bind (_starttrace _endtrace _starttrace1 _endtrace1 _starttrace2 _endtrace2 _starttrace3 _endtrace3) (CallFunction|GetLineTracesSpawnLocation))
  (bind _ac_lasercomp (Variables|Default|GetAC_LaserComp))
  (switch Utilities|FlowControl|Switch|SwitchonENUM_PrismState (Variables|Default|GetENUM_PrismState)
    (:NewEnumerator1
      (Default|SpawnLaserPrisme _ac_lasercomp _starttrace _endtrace false))
    (:NewEnumerator2
      (Default|SpawnLaserPrisme _ac_lasercomp _starttrace1 _endtrace1 false))
    (:NewEnumerator3
      (Default|SpawnLaserPrisme _ac_lasercomp _starttrace2 _endtrace2 false))
    (:NewEnumerator5
      (Default|SpawnLaserPrisme _ac_lasercomp "0, 0, 0" "0, 0, 0" true))))

(fn EventInteractionBouton
  (Utilities|FlowControl|FlipFlop
    (:A
      _)
    (:B
      (Utilities|Time|PauseTimerbyHandle (Variables|Default|GetLaserTimer))))
  (CallFunction|SwitchonSpawnPointEvent))

(fn SpawnSoundWave
  (bind (_starttrace _endtrace _starttrace1 _endtrace1 _starttrace2 _endtrace2 _starttrace3 _endtrace3) (CallFunction|GetSoundWaveSpawnLocation))
  (bind _ac_soundwave (Variables|Default|GetAC_SoundWave))
  (switch Utilities|FlowControl|Switch|SwitchonENUM_PrismState (Variables|Default|GetENUM_PrismState)
    (:NewEnumerator1
      (Default|SpawnSoundWave _ac_soundwave (Math|Transform|MakeTransform _starttrace (Math|Conversions|RotationFromXVector _endtrace) "1.000000,1.000000,1.000000")))
    (:NewEnumerator2
      (Default|SpawnSoundWave _ac_soundwave (Math|Transform|MakeTransform _starttrace1 (Math|Conversions|RotationFromXVector _endtrace1) "1.000000,1.000000,1.000000")))
    (:NewEnumerator3
      (Default|SpawnSoundWave _ac_soundwave (Math|Transform|MakeTransform _starttrace2 (Math|Conversions|RotationFromXVector _endtrace2) "1.000000,1.000000,1.000000")))
    (:NewEnumerator4
      (Default|SpawnSoundWave _ac_soundwave (Math|Transform|MakeTransform _starttrace3 (Math|Conversions|RotationFromXVector _endtrace3) "1.000000,1.000000,1.000000")))))

(fn SetRelativeSpawnPoint
  (bind _spawnlaserpoint0 (Variables|Default|GetSpawnLaserPoint0))
  (bind _returnvalue (Math|Vector|GetForwardVector _spawnlaserpoint0))
  (bind _returnvalue_2 (Math|Conversions|RotationFromXVector _returnvalue))
  (switch Utilities|FlowControl|Switch|SwitchonENUM_PrismState (Variables|Default|GetENUM_PrismState)
    (:NewEnumerator1
      (Transformation|SetRelativeRotation (Variables|Default|GetPrism) _returnvalue_2 false false)
      (Variables|Default|SetEndRotation _returnvalue_2))
    (:NewEnumerator2
      (Transformation|SetRelativeRotation (Variables|Default|GetPrism) (Math|Conversions|RotationFromXVector (Math|Vector|GetForwardVector (Variables|Default|GetSpawnLaserPoint1))) false false)
      (Variables|Default|SetEndRotation (Math|Rotator|MakeRotator 0.0 0.0 (+ (.yaw (Variables|Default|GetEndRotation)) 9e+01))))
    (:NewEnumerator3
      (Transformation|SetRelativeRotation (Variables|Default|GetPrism) (Math|Conversions|RotationFromXVector (Math|Vector|GetForwardVector (Variables|Default|GetSpawnLaserPoint2))) false false)
      (Variables|Default|SetEndRotation (Math|Rotator|MakeRotator 0.0 0.0 (+ (.yaw (Variables|Default|GetEndRotation)) 1.8e+02))))
    (:NewEnumerator4
      (Transformation|SetRelativeRotation (Variables|Default|GetPrism) (Math|Conversions|RotationFromXVector (Math|Vector|GetForwardVector (Variables|Default|GetSpawnLaserPoint3))) false false)
      (Variables|Default|SetEndRotation (Math|Rotator|MakeRotator 0.0 0.0 (+ (.yaw (Variables|Default|GetEndRotation)) 2.7e+02))))))

(fn GetSoundWaveSpawnLocation
  (bind _spawnlaserpoint3 (Variables|Default|GetSpawnLaserPoint3))
  (bind _spawnlaserpoint1 (Variables|Default|GetSpawnLaserPoint1))
  (bind _spawnlaserpoint0 (Variables|Default|GetSpawnLaserPoint0))
  (bind _spawnlaserpoint2 (Variables|Default|GetSpawnLaserPoint2))
  (bind _returnvalue (Transformation|GetWorldLocation _spawnlaserpoint2))
  (bind _returnvalue_2 (Transformation|GetWorldLocation _spawnlaserpoint0))
  (bind _returnvalue_3 (Transformation|GetWorldLocation _spawnlaserpoint1))
  (bind _returnvalue_4 (Transformation|GetWorldLocation _spawnlaserpoint3))
  (return _returnvalue_2 (+ _returnvalue_2 (* (Math|Vector|GetForwardVector (Transformation|GetWorldRotation _spawnlaserpoint0)) (LocalVariables|GetShockwaveOffset))) _returnvalue_3 (+ _returnvalue_3 (* (Math|Vector|GetForwardVector (Transformation|GetWorldRotation _spawnlaserpoint1)) (LocalVariables|GetShockwaveOffset))) _returnvalue (+ _returnvalue (* (Math|Vector|GetForwardVector (Transformation|GetWorldRotation _spawnlaserpoint2)) (LocalVariables|GetShockwaveOffset))) _returnvalue_4 (+ _returnvalue_4 (* (Math|Vector|GetForwardVector (Transformation|GetWorldRotation _spawnlaserpoint3)) (LocalVariables|GetShockwaveOffset)))))

(fn SetPrismRelativeRotation
  (bind _prism (Variables|Default|GetPrism))
  (switch Utilities|FlowControl|Switch|SwitchonENUM_PrismState (Variables|Default|GetENUM_PrismState)
    (:NewEnumerator1
      (Transformation|SetRelativeRotation _prism "0,-90.000000, 0" false false))
    (:NewEnumerator2
      (Transformation|SetRelativeRotation _prism "0,-180.000000, 0" false false))
    (:NewEnumerator3
      (Transformation|SetRelativeRotation _prism "0,-270.000000, 0" false false))
    (:NewEnumerator4
      (Transformation|SetRelativeRotation _prism "0.000000,-360.000000, 0" false false))))

(fn SwitchMatonPrismToolTip
  (switch Utilities|FlowControl|Switch|SwitchonENUM_PrismState (Variables|Default|GetENUM_PrismState)))

(fn SetSpawnPointsRelativeHeight
  (if (Variables|Default|GetisLaser?)
    (Transformation|AddLocalOffset (Variables|Default|GetSpawnLaserPoint0) "10.000000,0.000000,-6.000000" false false)
    (else
      (Transformation|AddLocalOffset (Variables|Default|GetSpawnLaserPoint0) "0, 0, 0" false false))))