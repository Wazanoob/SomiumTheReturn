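; Hub door Blueprint with four sliding panels that open and close through the DoorAnimation timeline, lerping their relative Y or Z positions.
; Player overlap plays or reverses it, unless the door is flagged as first-level or laser-driven.
; BeginPlay auto-plays it after a delay when the GameInstance LevelCount matches the door's enum; FinalDoor and InteractionCapteurTuto trigger it directly.
; UnlockDoorHHUB has no effect; spline-placement helpers are never called here.
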(event OnComponentBeginOverlap(Box)
  (params (OverlappedComponent :type Primitive%20Component%20Object%20Reference) (OtherActor :type Actor%20Object%20Reference) (OtherComp :type Primitive%20Component%20Object%20Reference) (OtherBodyIndex :type Integer) (bFromSweep :type Boolean) (SweepResult :type Hit%20Result%20Structure%20%28by%20ref%29))
  (if (Actor|ActorHasTag OtherActor "Joueur")
    (if (not (Variables|Default|GetIsFirstLevelDoor))
      (if (not (Variables|Default|GetWorkWithLaser))
        (CallFunction|PlayDoorAnim)
        (Variables|Default|SetIsDoorClosed? true)))))

(event OnComponentEndOverlap(Box)
  (params (OverlappedComponent :type Primitive%20Component%20Object%20Reference) (OtherActor :type Actor%20Object%20Reference) (OtherComp :type Primitive%20Component%20Object%20Reference) (OtherBodyIndex :type Integer))
  (if (Actor|ActorHasTag OtherActor "Joueur")
    (if (not (Variables|Default|GetIsFirstLevelDoor))
      (if (not (Variables|Default|GetWorkWithLaser))
        (CallFunction|AnimClosed)
        (Variables|Default|SetIsDoorClosed? false)))))

(event Custom|DoorMovementTimelineAnswer
  (Timeline|Timeline_0 Reverse))

(event Custom|DoorMouvementTimeline
  (Timeline|Timeline_0 Play))

(event Custom|PlayDoorAnim
  (bind _leftdoor (Variables|Default|GetLeftDoor))
  (bind _downdoor (Variables|Default|GetDownDoor))
  (bind _rightdoor (Variables|Default|GetRightDoor))
  (bind _topdoor (Variables|Default|GetTopDoor))
  (bind _leftdoor_2 (Variables|Default|GetLeftDoor))
  (bind _rightdoor_2 (Variables|Default|GetRightDoor))
  (bind _downdoor_2 (Variables|Default|GetDownDoor))
  (bind _topdoor_2 (Variables|Default|GetTopDoor))
  (bind _relativelocation (Variables|/Script/Engine.SceneComponent|GetRelativeLocation _leftdoor))
  (bind _relativelocation_2 (Variables|/Script/Engine.SceneComponent|GetRelativeLocation _rightdoor_2))
  (bind _relativelocation_3 (Variables|/Script/Engine.SceneComponent|GetRelativeLocation _rightdoor))
  (bind _relativelocation_4 (Variables|/Script/Engine.SceneComponent|GetRelativeLocation _downdoor))
  (bind _relativelocation_5 (Variables|/Script/Engine.SceneComponent|GetRelativeLocation _topdoor))
  (bind _relativelocation_6 (Variables|/Script/Engine.SceneComponent|GetRelativeLocation _leftdoor_2))
  (bind _relativelocation_7 (Variables|/Script/Engine.SceneComponent|GetRelativeLocation _downdoor_2))
  (bind _relativelocation_8 (Variables|/Script/Engine.SceneComponent|GetRelativeLocation _topdoor_2))
  (bind (_direction _bottomdoor _topdoor_3 _rightdoor_3 _leftdoor_3) (Timeline|DoorAnimation Play)
    (:Update
      (if (Variables|Default|GetIsDoorClosed?)
        (Utilities|FlowControl|Sequence
          (:then_0
            (Transformation|SetRelativeLocation _downdoor_2 (Math|Vector|MakeVector (.x _relativelocation_7) (.y _relativelocation_7) (Math|Float|Lerp (.z _relativelocation_7) (Variables|Default|GetBottomDoorPos) _bottomdoor)) false false))
          (:then_1
            (Transformation|SetRelativeLocation _topdoor_2 (Math|Vector|MakeVector (.x _relativelocation_8) (.y _relativelocation_8) (Math|Float|Lerp (.z _relativelocation_8) (Variables|Default|GetTopDoorPos) _topdoor_3)) false false))
          (:then_2
            (Transformation|SetRelativeLocation _rightdoor (Math|Vector|MakeVector (.x _relativelocation_3) (Math|Float|Lerp (.y _relativelocation_3) (Variables|Default|GetRightDoorPos) _rightdoor_3) (.z _relativelocation_3)) false false))
          (:then_3
            (Transformation|SetRelativeLocation _leftdoor (Math|Vector|MakeVector (.x _relativelocation) (Math|Float|Lerp (.y _relativelocation) (Variables|Default|GetLeftDoorPos) _leftdoor_3) (.z _relativelocation)) false false)))
        (else
          (Utilities|FlowControl|Sequence
            (:then_0
              (Transformation|SetRelativeLocation _downdoor (Math|Vector|MakeVector (.x _relativelocation_4) (.y _relativelocation_4) (Math|Float|Lerp 0.0 (.z _relativelocation_4) _bottomdoor)) false false))
            (:then_1
              (Transformation|SetRelativeLocation _topdoor (Math|Vector|MakeVector (.x _relativelocation_5) (.y _relativelocation_5) (Math|Float|Lerp 0.0 (.z _relativelocation_5) _topdoor_3)) false false))
            (:then_2
              (Transformation|SetRelativeLocation _rightdoor_2 (Math|Vector|MakeVector (.x _relativelocation_2) (Math|Float|Lerp 0.0 (.y _relativelocation_2) _rightdoor_3) (.z _relativelocation_2)) false false))
            (:then_3
              (Transformation|SetRelativeLocation _leftdoor_2 (Math|Vector|MakeVector (.x _relativelocation_6) (Math|Float|Lerp 0.0 (.y _relativelocation_6) _leftdoor_3) (.z _relativelocation_6)) false false))))))))

(event Custom|AnimClosed
  (bind _leftdoor (Variables|Default|GetLeftDoor))
  (bind _downdoor (Variables|Default|GetDownDoor))
  (bind _rightdoor (Variables|Default|GetRightDoor))
  (bind _topdoor (Variables|Default|GetTopDoor))
  (bind _leftdoor_2 (Variables|Default|GetLeftDoor))
  (bind _rightdoor_2 (Variables|Default|GetRightDoor))
  (bind _downdoor_2 (Variables|Default|GetDownDoor))
  (bind _topdoor_2 (Variables|Default|GetTopDoor))
  (bind _relativelocation (Variables|/Script/Engine.SceneComponent|GetRelativeLocation _leftdoor))
  (bind _relativelocation_2 (Variables|/Script/Engine.SceneComponent|GetRelativeLocation _rightdoor_2))
  (bind _relativelocation_3 (Variables|/Script/Engine.SceneComponent|GetRelativeLocation _rightdoor))
  (bind _relativelocation_4 (Variables|/Script/Engine.SceneComponent|GetRelativeLocation _downdoor))
  (bind _relativelocation_5 (Variables|/Script/Engine.SceneComponent|GetRelativeLocation _topdoor))
  (bind _relativelocation_6 (Variables|/Script/Engine.SceneComponent|GetRelativeLocation _leftdoor_2))
  (bind _relativelocation_7 (Variables|/Script/Engine.SceneComponent|GetRelativeLocation _downdoor_2))
  (bind _relativelocation_8 (Variables|/Script/Engine.SceneComponent|GetRelativeLocation _topdoor_2))
  (bind (_direction _bottomdoor _topdoor_3 _rightdoor_3 _leftdoor_3) (Timeline|DoorAnimation Reverse)
    (:Update
      (if (Variables|Default|GetIsDoorClosed?)
        (Utilities|FlowControl|Sequence
          (:then_0
            (Transformation|SetRelativeLocation _downdoor_2 (Math|Vector|MakeVector (.x _relativelocation_7) (.y _relativelocation_7) (Math|Float|Lerp (.z _relativelocation_7) (Variables|Default|GetBottomDoorPos) _bottomdoor)) false false))
          (:then_1
            (Transformation|SetRelativeLocation _topdoor_2 (Math|Vector|MakeVector (.x _relativelocation_8) (.y _relativelocation_8) (Math|Float|Lerp (.z _relativelocation_8) (Variables|Default|GetTopDoorPos) _topdoor_3)) false false))
          (:then_2
            (Transformation|SetRelativeLocation _rightdoor (Math|Vector|MakeVector (.x _relativelocation_3) (Math|Float|Lerp (.y _relativelocation_3) (Variables|Default|GetRightDoorPos) _rightdoor_3) (.z _relativelocation_3)) false false))
          (:then_3
            (Transformation|SetRelativeLocation _leftdoor (Math|Vector|MakeVector (.x _relativelocation) (Math|Float|Lerp (.y _relativelocation) (Variables|Default|GetLeftDoorPos) _leftdoor_3) (.z _relativelocation)) false false)))
        (else
          (Utilities|FlowControl|Sequence
            (:then_0
              (Transformation|SetRelativeLocation _downdoor (Math|Vector|MakeVector (.x _relativelocation_4) (.y _relativelocation_4) (Math|Float|Lerp 0.0 (.z _relativelocation_4) _bottomdoor)) false false))
            (:then_1
              (Transformation|SetRelativeLocation _topdoor (Math|Vector|MakeVector (.x _relativelocation_5) (.y _relativelocation_5) (Math|Float|Lerp 0.0 (.z _relativelocation_5) _topdoor_3)) false false))
            (:then_2
              (Transformation|SetRelativeLocation _rightdoor_2 (Math|Vector|MakeVector (.x _relativelocation_2) (Math|Float|Lerp 0.0 (.y _relativelocation_2) _rightdoor_3) (.z _relativelocation_2)) false false))
            (:then_3
              (Transformation|SetRelativeLocation _leftdoor_2 (Math|Vector|MakeVector (.x _relativelocation_6) (Math|Float|Lerp 0.0 (.y _relativelocation_6) _leftdoor_3) (.z _relativelocation_6)) false false))))))))

(event Custom|FinalDoor
  (CallFunction|UnlockDoorHHUB 0 2)
  (CallFunction|PlayDoorAnim))

(event EventBeginPlay
  (bind _asbp_my_game_instance (Utilities|Casting|CastToBP_MyGameInstance (Game|GetGameInstance)))
  (Variables|Default|SetAs%20BP%20My%20Game%20Instance _asbp_my_game_instance)
  (switch Utilities|FlowControl|Switch|SwitchonEnum_Level (Variables|Default|GetENUM_DoorPick)
    (:NewEnumerator0
      (if (== (Variables|/Game/OldSomium/Blueprints/BP_MyGameInstance.BP_MyGameInstance_C|GetLevelCount (Variables|Default|GetAs%20BP%20My%20Game%20Instance)) 2)
        _))
    (:NewEnumerator1
      (if (== (Variables|/Game/OldSomium/Blueprints/BP_MyGameInstance.BP_MyGameInstance_C|GetLevelCount (Variables|Default|GetAs%20BP%20My%20Game%20Instance)) 0)
        (CallFunction|UnlockDoorHHUB)
        (Utilities|FlowControl|Delay 22.0)
        (CallFunction|PlayDoorAnim)))
    (:NewEnumerator2
      (if (== (Variables|/Game/OldSomium/Blueprints/BP_MyGameInstance.BP_MyGameInstance_C|GetLevelCount (Variables|Default|GetAs%20BP%20My%20Game%20Instance)) 1)
        (CallFunction|UnlockDoorHHUB 0 1)
        (Utilities|FlowControl|Delay 6.0)
        (CallFunction|PlayDoorAnim)))))

(event EventInteractionCapteurTuto
  (CallFunction|PlayDoorAnim))

(fn ConstructionScript)

(fn MakeDoorTimeline
  (params (TimelineRef :type Float%20%28double-precision%29) (SplineInput :type Spline%20Component%20Object%20Reference) (DoorInput :type Scene%20Component%20Object%20Reference))
  (Transformation|SetWorldLocation DoorInput (Spline|GetLocationatDistanceAlongSpline SplineInput (* TimelineRef (Spline|GetSplineLength SplineInput)) "World") false false))

(fn SetPlateFormLoc&Rot
  (params (DoorInput :type Scene%20Component%20Object%20Reference) (SplineInput :type Spline%20Component%20Object%20Reference))
  (Transformation|SetWorldLocation DoorInput (Spline|GetLocationatDistanceAlongSpline SplineInput 0.0 "World") false false))

(fn UnlockDoorHHUB
  (params (ConcurrentLevel :type Integer) (LevelToOpen :type Integer))
  (bind _returnvalue (Game|GetCurrentLevelName true))
  (if (and (Utilities|Enum|Equal(Enum) _returnvalue "HUB-HP") (== ConcurrentLevel LevelToOpen))
    (return)))