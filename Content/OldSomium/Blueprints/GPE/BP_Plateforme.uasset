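; Spline-riding platform puzzle element that shuttles between two ends when hit by a sonic wave projectile.
; PlateformeType selects up to three meshes at construction, all driven along their splines by one timeline through a FlipFlop.
; Hits count only at the Reachable end, ripple a distortion material from the impact and message AttachedPlateforme; InteractionPlateforme bypasses that check.
; Movement lights the attached rail, with slide sounds and emissive material swaps.
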(event Custom|TimelinePingPong
  ;[1 1 1] On Onde Sonore Hit platform
  (Utilities|FlowControl|FlipFlop
    (:A
      (CallFunction|PlateformMouvementTimeline))
    (:B
      (CallFunction|PlatformMovementTimelineAnswer))))

(event Custom|PlateformMouvementTimeline
  ;[1 1 1] Plateformes Aller-retour
  (Variables|Default|SetPosition%20Plateforme%20A false)
  (if (Utilities|Enum|Equal(Enum) (Variables|Default|GetPlateformeAorB) "NewEnumerator0")
    (Variables|Default|SetReachable? false)
    (else
      (Variables|Default|SetReachable? true)))
  (Variables|Default|SetMoving true)
  (Default|LightRails (Variables|Default|GetAttached%20Rail))
  (bind _returnvalue (Audio|SpawnSound2D "/Game/FirstPerson/FX/SFX/Sound/Platforms/SC_Plateforme_Slide.SC_Plateforme_Slide" 1.0 1.0 0.0 0))
  (bind _traveldistance (Timeline|Timeline_0 Play)
    (:Update
      (CallFunction|SwitchonPlateformeType _traveldistance)
      (Utilities|FlowControl|DoOnce false :!label _label
        (:Completed
          (Audio|Components|Audio|Stop _returnvalue)
          (CallFunction|SetPlateformMaterialEmissive))))
    (:Finished
      (Variables|Default|SetMoving false)
      (bind _returnvalue_2 (Audio|SpawnSound2D "/Game/FirstPerson/FX/SFX/Sound/Platforms/SC_Plateforme_Lock.SC_Plateforme_Lock" 1.0 1.0 0.0 0))
      (Audio|Components|Audio|Stop _returnvalue_2)
      (CallFunction|SetPlateformMaterialNotEmissive)
      (Default|UnlightRails (Variables|Default|GetAttached%20Rail))
      (goto _label Reset))))

(event Custom|PlatformMovementTimelineAnswer
  ;[1 1 1] Plateformes Aller-retour
  (Variables|Default|SetPosition%20Plateforme%20A true)
  (if (Utilities|Enum|Equal(Enum) (Variables|Default|GetPlateformeAorB) "NewEnumerator0")
    (Variables|Default|SetReachable? true)
    (else
      (Variables|Default|SetReachable? false)))
  (Variables|Default|SetMoving true)
  (Default|LightRails (Variables|Default|GetAttached%20Rail))
  (bind _traveldistance (Timeline|Timeline_0 Reverse)
    (:Update
      (CallFunction|SwitchonPlateformeType _traveldistance)
      (Utilities|FlowControl|DoOnce false :!label _label
        (:Completed
          (Audio|Components|Audio|Stop (stale Custom|PlateformMouvementTimeline _returnvalue))
          (CallFunction|SetPlateformMaterialEmissive))))
    (:Finished
      (Variables|Default|SetMoving false)
      (bind _returnvalue (Audio|SpawnSound2D "/Game/FirstPerson/FX/SFX/Sound/Platforms/SC_Plateforme_Lock.SC_Plateforme_Lock" 1.0 1.0 0.0 0))
      (Audio|Components|Audio|Stop _returnvalue)
      (CallFunction|SetPlateformMaterialNotEmissive)
      (Default|UnlightRails (Variables|Default|GetAttached%20Rail))
      (goto _label Reset))))

(event Custom|EventHit
  (params (HitLocation :type Vector) (HitActor :type Hit%20Result%20Structure))
  (bind _hitcomponent (Collision|BreakHitResult HitActor))
  ;[1 1 1] SET DYNAMIC MATERIAL/ ORIENTER SONIC WAVE ON PLATFORM / SWITCH ON PLATEFORME INDEX
  (Utilities|FlowControl|Sequence
    (:then_0
      (if (== _hitcomponent (Variables|Default|GetPlateforme))
        (bind _returnvalue (Rendering|Material|CreateDynamicMaterialInstance (Variables|Default|GetPlateforme) 1 "/Game/FirstPerson/FX/VFX/IES/IES_Material/MA_WaveDistortion_Inst.MA_WaveDistortion_Inst" "None" :!class /Script/Engine.PrimitiveComponent))
        (bind _newtrack_0 (Timeline|Timeline_2 PlayFromStart)
          (:Update
            (Rendering|Material|SetVectorParameterValue _returnvalue "Position" (Math|Conversions|ToLinearColor(Vector) HitLocation) :!class /Script/Engine.MaterialInstanceDynamic)
            (Rendering|Material|SetScalarParameterValue _returnvalue "Radius" (* _newtrack_0 1.5e+03) :!class /Script/Engine.MaterialInstanceDynamic)))))
    (:then_1
      (if (== _hitcomponent (Variables|Default|GetPlateforme1))
        (bind _returnvalue_2 (Rendering|Material|CreateDynamicMaterialInstance (Variables|Default|GetPlateforme1) 1 "/Game/FirstPerson/FX/VFX/IES/IES_Material/MA_WaveDistortion_Inst.MA_WaveDistortion_Inst" "None" :!class /Script/Engine.PrimitiveComponent))
        (bind _newtrack_0_2 (Timeline|Timeline_3 PlayFromStart)
          (:Update
            (Rendering|Material|SetVectorParameterValue _returnvalue_2 "Position" (Math|Conversions|ToLinearColor(Vector) HitLocation) :!class /Script/Engine.MaterialInstanceDynamic)
            (Rendering|Material|SetScalarParameterValue _returnvalue_2 "Radius" (* _newtrack_0_2 1.5e+03) :!class /Script/Engine.MaterialInstanceDynamic)))))
    (:then_2
      (if (== _hitcomponent (Variables|Default|GetPlateforme2))
        (bind _returnvalue_3 (Rendering|Material|CreateDynamicMaterialInstance (Variables|Default|GetPlateforme2) 1 "/Game/FirstPerson/FX/VFX/IES/IES_Material/MA_WaveDistortion_Inst.MA_WaveDistortion_Inst" "None" :!class /Script/Engine.PrimitiveComponent))
        (bind _newtrack_0_3 (Timeline|Timeline_4 PlayFromStart)
          (:Update
            (Rendering|Material|SetVectorParameterValue _returnvalue_3 "Position" (Math|Conversions|ToLinearColor(Vector) HitLocation) :!class /Script/Engine.MaterialInstanceDynamic)
            (Rendering|Material|SetScalarParameterValue _returnvalue_3 "Radius" (* _newtrack_0_3 1.5e+03) :!class /Script/Engine.MaterialInstanceDynamic)))))))

(event EventBeginPlay
  (CallFunction|SetPlateformeAorB))

(event Collision|EventHit
  (params (MyComp :type Primitive%20Component%20Object%20Reference) (Other :type Actor%20Object%20Reference) (OtherComp :type Primitive%20Component%20Object%20Reference) (bSelfMoved :type Boolean) (HitLocation :type Vector :default "0, 0, 0") (HitNormal :type Vector :default "0, 0, 0") (NormalImpulse :type Vector :default "0, 0, 0") (Hit :type Hit%20Result%20Structure%20%28by%20ref%29))
  ;[1 1 1] On Onde Sonore Hit platform
  (Utilities|IsValid (.AsBP%20Sonic%20Wave%20Projectile (Utilities|Casting|CastToBP_SonicWaveProjectile Other))
    (:Is%20Valid
      (if (Variables|Default|GetReachable?)
        ;;[1 1 1] pour material sur plateformes
        (CallFunction|EventHit HitLocation Hit)
        (Audio|SpawnSoundAttached "/Game/FirstPerson/FX/SFX/Sound/Platforms/SC_Plateforme_WaveHit.SC_Plateforme_WaveHit" (Variables|Default|GetPlateforme) "None" "0, 0, 0" "0, 0, 0" "KeepRelativeOffset" false 1.0 1.0 0.0 0 0)
        (if (not (Variables|Default|GetMoving))
          (CallFunction|TimelinePingPong)
          (Class|BPInteraction|InteractionPlateforme(Message) (Variables|Default|GetAttachedPlateforme)))))))

(event EventInteractionPlateforme
  ;[1 1 1] On Onde Sonore Hit platform
  (if (not (Variables|Default|GetMoving))
    (CallFunction|TimelinePingPong)))

(event Input|KeyboardEvents|^
  (params (Key :type Key%20Structure))
  (:Pressed
    (Development|ExecuteConsoleCommand "stat FPS" 0)))

(fn ConstructionScript
  (CallFunction|MakePlateformeSystem))

(fn SetPlateformeLocation&Rotation
  (params (PlateFormeInput :type Scene%20Component%20Object%20Reference) (SplineInput :type Spline%20Component%20Object%20Reference))
  (bind _returnvalue (Spline|GetRotationatDistanceAlongSpline SplineInput 0.0 "Local"))
  (Transformation|SetRelativeRotation PlateFormeInput (Math|Rotator|MakeRotator (.roll _returnvalue) 0.0 (.yaw _returnvalue)) false false)
  (Transformation|SetWorldLocation PlateFormeInput (Spline|GetLocationatDistanceAlongSpline SplineInput 0.0 "World") false false))

(fn MakePlateformeTimeline
  (params (PlateformeInput :type Scene%20Component%20Object%20Reference) (SplineInput :type Spline%20Component%20Object%20Reference) (TimelineRef :type Float%20%28double-precision%29))
  (bind _returnvalue (Spline|GetSplineLength SplineInput))
  (bind _returnvalue_2 (* TimelineRef _returnvalue))
  (Transformation|SetWorldLocation (LocalVariables|GetPlateFormeInput) (Spline|GetLocationatDistanceAlongSpline SplineInput _returnvalue_2 "World") false false)
  (Transformation|SetRelativeRotation (LocalVariables|GetPlateFormeInput) (Spline|GetRotationatDistanceAlongSpline SplineInput _returnvalue_2 "Local") false false))

(fn SwitchonPlateformeType
  (params (TimelineRef :type Float%20%28double-precision%29))
  (switch Utilities|FlowControl|Switch|SwitchonENUM_PlatformType (Variables|Default|GetPlateformeType)
    (:NewEnumerator0
      (CallFunction|MakePlateformeTimeline (Variables|Default|GetPlateforme) (Variables|Default|GetSpline) TimelineRef))
    (:NewEnumerator1
      (CallFunction|MakePlateformeTimeline (Variables|Default|GetPlateforme1) (Variables|Default|GetSpline1) TimelineRef))
    (:NewEnumerator2
      (CallFunction|MakePlateformeTimeline (Variables|Default|GetPlateforme2) (Variables|Default|GetSpline2) TimelineRef))
    (:NewEnumerator3
      (Utilities|FlowControl|Sequence
        (:then_0
          (CallFunction|MakePlateformeTimeline (Variables|Default|GetPlateforme) (Variables|Default|GetSpline) TimelineRef))
        (:then_1
          (CallFunction|MakePlateformeTimeline (Variables|Default|GetPlateforme1) (Variables|Default|GetSpline1) TimelineRef))))
    (:NewEnumerator4
      (Utilities|FlowControl|Sequence
        (:then_0
          (CallFunction|MakePlateformeTimeline (Variables|Default|GetPlateforme) (Variables|Default|GetSpline) TimelineRef))
        (:then_1
          (CallFunction|MakePlateformeTimeline (Variables|Default|GetPlateforme2) (Variables|Default|GetSpline2) TimelineRef))))
    (:NewEnumerator5
      (Utilities|FlowControl|Sequence :!label _label
        (:then_0
          (CallFunction|MakePlateformeTimeline (Variables|Default|GetPlateforme1) (Variables|Default|GetSpline1) TimelineRef))
        (:then_1
          (CallFunction|MakePlateformeTimeline (Variables|Default|GetPlateforme2) (Variables|Default|GetSpline2) TimelineRef))))
    (:NewEnumerator6
      (CallFunction|MakePlateformeTimeline (Variables|Default|GetPlateforme) (Variables|Default|GetSpline) TimelineRef)
      (goto _label))))

(fn SetAllPlateformsLoc&Rot
  (Utilities|FlowControl|Sequence
    (:then_0
      (CallFunction|SetPlateformeLocation&Rotation (Variables|Default|GetPlateforme) (Variables|Default|GetSpline)))
    (:then_1
      (CallFunction|SetPlateformeLocation&Rotation (Variables|Default|GetPlateforme1) (Variables|Default|GetSpline1)))
    (:then_2
      (CallFunction|SetPlateformeLocation&Rotation (Variables|Default|GetPlateforme2) (Variables|Default|GetSpline2)))))

(fn MakePlateformeSystem
  (switch Utilities|FlowControl|Switch|SwitchonENUM_PlatformType (Variables|Default|GetPlateformeType)
    (:NewEnumerator0
      ;[1 1 1] P0
      (Components|StaticMesh|SetStaticMesh (Variables|Default|GetPlateforme) (Variables|Default|GetPlateformeAsset))
      (Components|DestroyComponent (Variables|Default|GetPlateforme1))
      (Components|DestroyComponent (Variables|Default|GetPlateforme2)))
    (:NewEnumerator1
      ;[1 1 1] P1
      (Components|StaticMesh|SetStaticMesh (Variables|Default|GetPlateforme1) (Variables|Default|GetPlateformeAsset))
      (Components|DestroyComponent (Variables|Default|GetPlateforme))
      (Components|DestroyComponent (Variables|Default|GetPlateforme2)))
    (:NewEnumerator2
      ;[1 1 1] P2
      (Components|StaticMesh|SetStaticMesh (Variables|Default|GetPlateforme2) (Variables|Default|GetPlateformeAsset))
      (Components|DestroyComponent (Variables|Default|GetPlateforme))
      (Components|DestroyComponent (Variables|Default|GetPlateforme1)))
    (:NewEnumerator3
      ;[1 1 1] P0 & P1
      (Components|StaticMesh|SetStaticMesh (Variables|Default|GetPlateforme) (Variables|Default|GetPlateformeAsset))
      (Components|StaticMesh|SetStaticMesh (Variables|Default|GetPlateforme1) (Variables|Default|GetPlateformeAsset))
      (Components|DestroyComponent (Variables|Default|GetPlateforme2)))
    (:NewEnumerator4
      ;[1 1 1] P0 & P2
      (Components|StaticMesh|SetStaticMesh (Variables|Default|GetPlateforme) (Variables|Default|GetPlateformeAsset))
      (Components|StaticMesh|SetStaticMesh (Variables|Default|GetPlateforme2) (Variables|Default|GetPlateformeAsset))
      (Components|DestroyComponent (Variables|Default|GetPlateforme1)))
    (:NewEnumerator5
      ;[1 1 1] P1 & P2
      (Components|StaticMesh|SetStaticMesh (Variables|Default|GetPlateforme1) (Variables|Default|GetPlateformeAsset))
      (Components|StaticMesh|SetStaticMesh (Variables|Default|GetPlateforme2) (Variables|Default|GetPlateformeAsset))
      (Components|DestroyComponent (Variables|Default|GetPlateforme)))
    (:NewEnumerator6
      ;[1 1 1] P0 & P1 & P2
      (Components|StaticMesh|SetStaticMesh (Variables|Default|GetPlateforme) (Variables|Default|GetPlateformeAsset))
      (Components|StaticMesh|SetStaticMesh (Variables|Default|GetPlateforme1) (Variables|Default|GetPlateformeAsset))
      (Components|StaticMesh|SetStaticMesh (Variables|Default|GetPlateforme2) (Variables|Default|GetPlateformeAsset)))
    (:NewEnumerator7
      ;[1 1 1] NONE
      (Components|DestroyComponent (Variables|Default|GetPlateforme))
      (Components|DestroyComponent (Variables|Default|GetPlateforme1))
      (Components|DestroyComponent (Variables|Default|GetPlateforme2)))))

(fn SetPlateformMaterialEmissive
  (bind _plateforme1 (Variables|Default|GetPlateforme1))
  (bind _plateforme (Variables|Default|GetPlateforme))
  (switch Utilities|FlowControl|Switch|SwitchonENUM_PlatformType (Variables|Default|GetPlateformeType)
    (:NewEnumerator0
      (Rendering|Material|SetMaterial _plateforme 2 "/Game/OldSomium/ART/Meshes/GPE/Plateformes/Good-one/M_GPE_Blocker_Emissive.M_GPE_Blocker_Emissive"))
    (:NewEnumerator1
      (Rendering|Material|SetMaterial _plateforme1 2 "/Game/OldSomium/ART/Meshes/GPE/Plateformes/Good-one/M_GPE_Blocker_Emissive.M_GPE_Blocker_Emissive"))
    (:NewEnumerator2
      (Rendering|Material|SetMaterial (Variables|Default|GetPlateforme2) 2 "/Game/OldSomium/ART/Meshes/GPE/Plateformes/Good-one/M_GPE_Blocker_Emissive.M_GPE_Blocker_Emissive"))
    (:NewEnumerator3
      (Rendering|Material|SetMaterial _plateforme 2 "/Game/OldSomium/ART/Meshes/GPE/Plateformes/Good-one/M_GPE_Blocker_Emissive.M_GPE_Blocker_Emissive"))
    (:NewEnumerator4
      (Rendering|Material|SetMaterial _plateforme 2 "/Game/OldSomium/ART/Meshes/GPE/Plateformes/Good-one/M_GPE_Blocker_Emissive.M_GPE_Blocker_Emissive"))
    (:NewEnumerator5
      (Rendering|Material|SetMaterial _plateforme1 2 "/Game/OldSomium/ART/Meshes/GPE/Plateformes/Good-one/M_GPE_Blocker_Emissive.M_GPE_Blocker_Emissive"))
    (:NewEnumerator6
      (Rendering|Material|SetMaterial _plateforme1 2 "/Game/OldSomium/ART/Meshes/GPE/Plateformes/Good-one/M_GPE_Blocker_Emissive.M_GPE_Blocker_Emissive"))))

(fn SetPlateformMaterialNotEmissive
  (bind _plateforme1 (Variables|Default|GetPlateforme1))
  (bind _plateforme (Variables|Default|GetPlateforme))
  (switch Utilities|FlowControl|Switch|SwitchonENUM_PlatformType (Variables|Default|GetPlateformeType)
    (:NewEnumerator0
      (Rendering|Material|SetMaterial _plateforme 2 "/Game/OldSomium/ART/Materials/Couleurs/M_Black.M_Black"))
    (:NewEnumerator1
      (Rendering|Material|SetMaterial _plateforme1 2 "/Game/OldSomium/ART/Materials/Couleurs/M_Black.M_Black"))
    (:NewEnumerator2
      (Rendering|Material|SetMaterial (Variables|Default|GetPlateforme2) 2 "/Game/OldSomium/ART/Materials/Couleurs/M_Black.M_Black"))
    (:NewEnumerator3
      (Rendering|Material|SetMaterial _plateforme 2 "/Game/OldSomium/ART/Materials/Couleurs/M_Black.M_Black"))
    (:NewEnumerator4
      (Rendering|Material|SetMaterial _plateforme 2 "/Game/OldSomium/ART/Materials/Couleurs/M_Black.M_Black"))
    (:NewEnumerator5
      (Rendering|Material|SetMaterial _plateforme1 2 "/Game/OldSomium/ART/Materials/Couleurs/M_Black.M_Black"))
    (:NewEnumerator6
      (Rendering|Material|SetMaterial _plateforme1 2 "/Game/OldSomium/ART/Materials/Couleurs/M_Black.M_Black"))))

(fn SetPlateformeAorB
  (switch Utilities|FlowControl|Switch|SwitchonENUM_Plateforme_AorB (Variables|Default|GetPlateformeAorB)
    (:NewEnumerator0
      (if (Variables|Default|GetPosition%20Plateforme%20A)
        (Variables|Default|SetReachable? true)
        (else
          (Variables|Default|SetReachable? false))))
    (:NewEnumerator1
      (if (Variables|Default|GetPosition%20Plateforme%20A)
        (Variables|Default|SetReachable? false)
        (else
          (Variables|Default|SetReachable? true))))))