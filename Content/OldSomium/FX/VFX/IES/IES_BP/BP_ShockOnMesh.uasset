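; BP_ShockOnMesh plays a shockwave distortion on its Sphere mesh from a hit location.
; The Hit event prints the location and creates a dynamic instance of MA_WaveDistortion_Inst on the sphere.
; A timeline then feeds that location into the material's Position parameter and grows Radius from its scaled track.
; The Condition flag is only ever set true, so it does not block retriggering.
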(event Custom|EventHit
  (params (InputPin :type Vector))
  (Variables|Default|SetCondition true)
  (if (Variables|Default|GetCondition)
    (Development|PrintText (Utilities|Text|ToText(String) InputPin))
    (bind _returnvalue (Rendering|Material|CreateDynamicMaterialInstance (Variables|Default|GetSphere) 0 "/Game/OldSomium/FX/VFX/IES/IES_Material/MA_WaveDistortion_Inst.MA_WaveDistortion_Inst" "None" :!class /Script/Engine.PrimitiveComponent))
    (bind _newtrack_0 (Timeline|Timeline_0 PlayFromStart)
      (:Update
        (Rendering|Material|SetVectorParameterValue _returnvalue "Position" (Math|Conversions|ToLinearColor(Vector) InputPin) :!class /Script/Engine.MaterialInstanceDynamic)
        (Rendering|Material|SetScalarParameterValue _returnvalue "Radius" (* _newtrack_0 1.5e+03) :!class /Script/Engine.MaterialInstanceDynamic))
      (:Finished
        (Variables|Default|SetCondition true)))))

(event Collision|EventHit
  (params (MyComp :type Primitive%20Component%20Object%20Reference) (Other :type Actor%20Object%20Reference) (OtherComp :type Primitive%20Component%20Object%20Reference) (bSelfMoved :type Boolean) (HitLocation :type Vector :default "0, 0, 0") (HitNormal :type Vector :default "0, 0, 0") (NormalImpulse :type Vector :default "0, 0, 0") (Hit :type Hit%20Result%20Structure%20%28by%20ref%29))
  (CallFunction|EventHit HitLocation))

(fn ConstructionScript)