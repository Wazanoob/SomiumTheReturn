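; BP_Line is a trigger actor in the VFX folder that passes a trace impact point to BP_ShockOnMesh, apparently as a test setup.
; A Box overlap fires a Camera-channel line trace from the SpringArm, ending at its world position with X multiplied by 1000 rather than along its forward vector.
; It draws persistent debug, prints the impact point and calls EventHit on any hit BP_ShockOnMesh.
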(event OnComponentBeginOverlap(Box)
  (params (OverlappedComponent :type Primitive%20Component%20Object%20Reference) (OtherActor :type Actor%20Object%20Reference) (OtherComp :type Primitive%20Component%20Object%20Reference) (OtherBodyIndex :type Integer) (bFromSweep :type Boolean) (SweepResult :type Hit%20Result%20Structure%20%28by%20ref%29))
  (bind _springarm (Variables|Default|GetSpringArm))
  (bind _returnvalue (Transformation|GetWorldLocation _springarm))
  (bind (_x _y _z) (Math|Vector|BreakVector _returnvalue))
  (bind _outhit (Collision|LineTraceByChannel _returnvalue (Math|Vector|MakeVector (* _x 1e+03) _y _z) "TraceTypeQuery2" false 0 "Persistent"))
  (bind _output_get (Variables|Default|SetImpact%20Point (.ImpactPoint (Collision|BreakHitResult _outhit))))
  (Development|PrintText (Utilities|Text|ToText(String) _output_get))
  (bind _asbp_shock_on_mesh (Utilities|Casting|CastToBP_ShockOnMesh (.HitActor (Collision|BreakHitResult _outhit))))
  (Default|EventHit _asbp_shock_on_mesh _output_get))

(event Custom|Test)

(event EventBeginPlay)

(event Collision|EventActorBeginOverlap
  (params (OtherActor :type Actor%20Object%20Reference)))

(event EventTick
  (params (DeltaSeconds :type Float%20%28single-precision%29)))

(fn ConstructionScript)