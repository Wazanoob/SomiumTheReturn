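; BP_WidgetFloating is a floating widget actor that displays the ID of a BP_Recepteur or BP_Scanner.
; On BeginPlay it reads the ID from its parent actor, falling back to an ActorIndependant reference, and sends it as text to its WBP_FréquenceAnim widget.
; Each Tick it rotates to face the cached player, but only while ActorIndependant is not valid, so independently linked instances keep their rotation.
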(event EventTick
  (params (DeltaSeconds :type Float%20%28single-precision%29))
  ;[1 1 1] Comment
  (Variables|Default|GetActorIndependant
    (:then)
    (:else
      (Transformation|SetActorRotation (Math|Rotator|FindLookatRotation (Transformation|GetActorLocation) (Transformation|GetActorLocation (Variables|Default|GetAs%20BP%20Player)))))))

(event EventBeginPlay
  (bind _returnvalue (Actor|GetParentActor))
  (bind _asbp_player (Utilities|Casting|CastToBP_Player (Game|GetPlayerCharacter 0)))
  (Variables|Default|SetAs%20BP%20Player _asbp_player)
  (bind _asbp_recepteur (Utilities|Casting|CastToBP_Recepteur _returnvalue)
    (:then
      (bind _aswbp_fréquence_anim (Utilities|Casting|CastToWBP_FréquenceAnim (UserInterface|GetWidget (Variables|Default|GetWidget))))
      (Default|UpdateText _aswbp_fréquence_anim (Utilities|Text|ToText(Integer) (Variables|/Game/Somium2/Blueprints/GPE/BP_Recepteur.BP_Recepteur_C|GetID _asbp_recepteur))))
    (:CastFailed
      (bind _asbp_scanner (Utilities|Casting|CastToBP_Scanner _returnvalue)
        (:then
          (bind _aswbp_fréquence_anim_2 (Utilities|Casting|CastToWBP_FréquenceAnim (UserInterface|GetWidget (Variables|Default|GetWidget))))
          (Default|UpdateText _aswbp_fréquence_anim_2 (Utilities|Text|ToText(Integer) (Variables|/Game/Somium2/Blueprints/GPE/BP_Scanner.BP_Scanner_C|GetID%20Scanner _asbp_scanner))))
        (:CastFailed
          (bind _actorindependant (Variables|Default|GetActorIndependant)
            (:then
              ;[1 1 1] Comment
              (bind _asbp_scanner_2 (Utilities|Casting|CastToBP_Scanner _actorindependant)
                (:then
                  (bind _aswbp_fréquence_anim_3 (Utilities|Casting|CastToWBP_FréquenceAnim (UserInterface|GetWidget (Variables|Default|GetWidget))))
                  (Default|UpdateText _aswbp_fréquence_anim_3 (Utilities|Text|ToText(Integer) (Variables|/Game/Somium2/Blueprints/GPE/BP_Scanner.BP_Scanner_C|GetID%20Scanner _asbp_scanner_2))))
                (:CastFailed
                  ;[1 1 1] Comment
                  (bind _asbp_recepteur_2 (Utilities|Casting|CastToBP_Recepteur _actorindependant))
                  (bind _aswbp_fréquence_anim_4 (Utilities|Casting|CastToWBP_FréquenceAnim (UserInterface|GetWidget (Variables|Default|GetWidget))))
                  (Default|UpdateText _aswbp_fréquence_anim_4 (Utilities|Text|ToText(Integer) (Variables|/Game/Somium2/Blueprints/GPE/BP_Recepteur.BP_Recepteur_C|GetID _asbp_recepteur_2))))))
            (:else)))))))

(fn ConstructionScript)