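; BP_GameMode is a game mode Blueprint that handles pausing and resuming the game.
; SetPause pauses the game, shows the mouse cursor and has the player character, cast to BP_Player, open its paused menu.
; Resume removes all widgets, unpauses and has BP_Player show the HUD again, without hiding the mouse cursor.
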(fn ConstructionScript)

(fn SetPause
  (Game|SetGamePaused true)
  (Variables|/Script/Engine.PlayerController|SetbShowMouseCursor (Game|GetPlayerController 0) true)
  (bind _asbp_player (Utilities|Casting|CastToBP_Player (Game|GetPlayerCharacter 0)))
  (Default|PausedMenu _asbp_player))

(fn Resume
  (Viewport|RemoveAllWidgets)
  (Game|SetGamePaused false)
  (bind _asbp_player (Utilities|Casting|CastToBP_Player (Game|GetPlayerCharacter 0)))
  (Default|HUD _asbp_player))