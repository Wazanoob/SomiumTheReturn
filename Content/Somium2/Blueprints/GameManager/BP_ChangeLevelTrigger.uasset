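; BP_ChangeLevelTrigger is a one-shot trigger box that resets the player's robot companion, apparently at a level transition.
; On player overlap it clears the SpecialQR references on player and robot and zeroes the player's robot target position.
; It hides and releases any object in the robot's storage, moves the robot to the SpawnPosition actor, then destroys itself.
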(event OnComponentBeginOverlap(TriggerBox)
  (params (OverlappedComponent :type Primitive%20Component%20Object%20Reference) (OtherActor :type Actor%20Object%20Reference) (OtherComp :type Primitive%20Component%20Object%20Reference) (OtherBodyIndex :type Integer) (bFromSweep :type Boolean) (SweepResult :type Hit%20Result%20Structure%20%28by%20ref%29))
  (bind _asbp_player (Utilities|Casting|CastToBP_Player OtherActor))
  (Variables|/Game/Somium2/Blueprints/Player/BP_Player.BP_Player_C|SetSpecialQR _asbp_player 0)
  (Variables|/Game/Somium2/Blueprints/Player/BP_Player.BP_Player_C|SetRobotTargetPosition _asbp_player "0, 0, 0")
  (Variables|/Game/Somium2/Blueprints/GPE/Robot_MSE-6/BP_Drone_MSE-6.BP_Drone_MSE-6_C|SetSpecialQR (Variables|/Game/Somium2/Blueprints/Player/BP_Player.BP_Player_C|GetMyRobotFriend _asbp_player) 0)
  (bind _mycarryingobject (Variables|/Game/Somium2/Blueprints/GPE/Robot_MSE-6/BP_Drone_Stockage.BP_Drone_Stockage_C|GetMyCarryingObject (Variables|/Game/Somium2/Blueprints/GPE/Robot_MSE-6/BP_Drone_MSE-6.BP_Drone_MSE-6_C|GetMyStockage (Variables|/Game/Somium2/Blueprints/Player/BP_Player.BP_Player_C|GetMyRobotFriend _asbp_player)))
    (:then
      (Rendering|SetActorHiddenInGame _mycarryingobject true)
      (Variables|/Game/Somium2/Blueprints/GPE/Robot_MSE-6/BP_Drone_Stockage.BP_Drone_Stockage_C|SetMyCarryingObject (Variables|/Game/Somium2/Blueprints/GPE/Robot_MSE-6/BP_Drone_MSE-6.BP_Drone_MSE-6_C|GetMyStockage (Variables|/Game/Somium2/Blueprints/Player/BP_Player.BP_Player_C|GetMyRobotFriend _asbp_player)) 0)
      (Variables|/Game/Somium2/Blueprints/GPE/Robot_MSE-6/BP_Drone_Stockage.BP_Drone_Stockage_C|SetIsCarryingObject (Variables|/Game/Somium2/Blueprints/GPE/Robot_MSE-6/BP_Drone_MSE-6.BP_Drone_MSE-6_C|GetMyStockage (Variables|/Game/Somium2/Blueprints/Player/BP_Player.BP_Player_C|GetMyRobotFriend _asbp_player)) false)
      (Development|PrintString "reset CarryingObject Robot"))
    (:else
      _))
  (Transformation|SetActorLocation (Variables|/Game/Somium2/Blueprints/Player/BP_Player.BP_Player_C|GetMyRobotFriend _asbp_player) (Transformation|GetActorLocation (Variables|Default|GetSpawnPosition)) false false)
  (Actor|DestroyActor))

(event EventBeginPlay)

(event Collision|EventActorBeginOverlap
  (params (OtherActor :type Actor%20Object%20Reference)))

(fn ConstructionScript)