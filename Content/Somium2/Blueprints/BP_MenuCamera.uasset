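; Menu camera that sways with the mouse and drives clicks on in-world widgets.
; BeginPlay shows and centers the cursor; Tick interpolates camera pitch and yaw from cursor offset, both measured against half the viewport width, and replays a world camera shake.
; Tick also moves the WidgetInteraction component to the cursor's visibility-trace hit point, and the Click action sends it left-button presses and releases.
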(event EventBeginPlay
  (bind _returnvalue (Viewport|GetViewportSize))
  (bind _returnvalue_2 (Class|GameplayStatics|GetPlayerControllerfromID))
  ;[1 1 1] Comment
  (Variables|/Script/Engine.PlayerController|SetbShowMouseCursor _returnvalue_2 true)
  (Variables|Default|SetRotationSpawn (Transformation|GetActorRotation))
  (Utilities|FlowControl|Delay 0.2)
  (Class|PlayerController|SetMouseLocation _returnvalue_2 (Math|Float|Truncate (/ (.x _returnvalue) 2.0)) (Math|Float|Truncate (/ (.y _returnvalue) 2.0))))

(event EventTick
  (params (DeltaSeconds :type Float%20%28single-precision%29))
  (bind _returnvalue (Transformation|GetActorRotation))
  (bind _returnvalue_2 (Viewport|GetViewportSize))
  (bind _returnvalue_3 (Utilities|Time|GetWorldDeltaSeconds))
  (bind _returnvalue_4 (Class|GameplayStatics|GetPlayerControllerfromID))
  (bind (_locationx _locationy) (Game|Player|GetMousePosition _returnvalue_4))
  (bind _returnvalue_5 (/ (.x _returnvalue_2) 2.0))
  ;[1 1 1] Comment
  (Camera|PlayWorldCameraShake 0 (Transformation|GetActorLocation) 1e+02 5e+02)
  (bind _output_get (Variables|Default|SetRotationSpawn (Math|Rotator|MakeRotator (.roll (Variables|Default|GetRotationSpawn)) (Math|Interpolation|FInterpTo (.pitch (Variables|Default|GetRotationSpawn)) (+ (.pitch _returnvalue) (* (/ (- _locationy _returnvalue_5) 4e+02) -1.0)) _returnvalue_3 5.0) (Math|Interpolation|FInterpTo (.yaw (Variables|Default|GetRotationSpawn)) (+ (.yaw _returnvalue) (/ (- _locationx _returnvalue_5) 2e+02)) _returnvalue_3 5.0))))
  (Transformation|SetWorldRotation (Variables|Default|GetCamera) (Math|Rotator|MakeRotator (.roll _output_get) (.pitch _output_get) (.yaw _output_get)) false false)
  (Transformation|SetWorldLocation (Variables|Default|GetWidgetInteraction) (.Location (Collision|BreakHitResult (.HitResult (Game|Player|GetHitResultUnderCursorbyChannel (Class|GameplayStatics|GetPlayerControllerfromID) "TraceTypeQuery1" true)))) false false))

(event Input|ActionEvents|InputActionClick
  (params (Key :type Key%20Structure :default "None"))
  (bind _widgetinteraction (Variables|Default|GetWidgetInteraction))
  ;[1 1 1] Comment
  (:Pressed
    (Class|WidgetInteractionComponent|PressPointerKey _widgetinteraction "LeftMouseButton"))
  (:Released
    (Class|WidgetInteractionComponent|ReleasePointerKey _widgetinteraction "LeftMouseButton")))

(fn ConstructionScript)