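; AC_MoveRobot is a player actor component that manages an Aura marker actor, apparently for indicating a robot move position.
; On BeginPlay it spawns the Aura at the owner's location, keeps a reference and hides it.
; EnableAura and DisableAura toggle its visibility.
; CheckRobotPosition only relocates the Aura to the given target, with no validation or robot movement.
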(event Custom|EnableAura
  (Rendering|SetActorHiddenInGame (Variables|Default|GetMyAura) false))

(event Custom|DisableAura
  (Rendering|SetActorHiddenInGame (Variables|Default|GetMyAura) true))

(event EventBeginPlay
  (bind _returnvalue (Game|SpawnActorfromClass (Variables|Default|GetAura) (Math|Conversions|ToTransform(Vector) (Transformation|GetActorLocation (Components|GetOwner))) "Undefined" 0 0))
  (bind _output_get (Variables|Default|SetMyAura _returnvalue))
  (Rendering|SetActorHiddenInGame _output_get true))

(fn CheckRobotPosition
  (params (TargetPosition :type Vector))
  (Transformation|SetActorLocation (Variables|Default|GetMyAura) TargetPosition false false))