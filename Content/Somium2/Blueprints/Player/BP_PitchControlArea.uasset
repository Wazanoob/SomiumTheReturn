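; BP_PitchControlArea is a trigger volume that lowers the pitch of the player's audio while BP_Player is inside its Box.
; Entering plays a timeline that lerps the player's AudioCurveSource pitch multiplier from normal down to a deeper value.
; Leaving reverses the same timeline, easing the pitch back to normal.
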(event OnComponentBeginOverlap(Box)
  (params (OverlappedComponent :type Primitive%20Component%20Object%20Reference) (OtherActor :type Actor%20Object%20Reference) (OtherComp :type Primitive%20Component%20Object%20Reference) (OtherBodyIndex :type Integer) (bFromSweep :type Boolean) (SweepResult :type Hit%20Result%20Structure%20%28by%20ref%29))
  (bind _asbp_player (Utilities|Casting|CastToBP_Player OtherActor))
  (Variables|Default|SetAudio%20Curve%20Source (Variables|/Game/Somium2/Blueprints/Player/BP_Player.BP_Player_C|GetAudioCurveSource _asbp_player))
  (bind _newtrack_0 (Timeline|Timeline_0 Play)
    (:Update
      (Audio|Components|Audio|SetPitchMultiplier (Variables|Default|GetAudio%20Curve%20Source) (Math|Float|Lerp 1.0 0.7 _newtrack_0)))))

(event OnComponentEndOverlap(Box)
  (params (OverlappedComponent :type Primitive%20Component%20Object%20Reference) (OtherActor :type Actor%20Object%20Reference) (OtherComp :type Primitive%20Component%20Object%20Reference) (OtherBodyIndex :type Integer))
  (bind _asbp_player (Utilities|Casting|CastToBP_Player OtherActor))
  (Variables|Default|SetAudio%20Curve%20Source (Variables|/Game/Somium2/Blueprints/Player/BP_Player.BP_Player_C|GetAudioCurveSource _asbp_player))
  (bind _newtrack_0 (Timeline|Timeline_0 Reverse)
    (:Update
      (Audio|Components|Audio|SetPitchMultiplier (Variables|Default|GetAudio%20Curve%20Source) (Math|Float|Lerp 1.0 0.7 _newtrack_0)))))

(fn ConstructionScript)