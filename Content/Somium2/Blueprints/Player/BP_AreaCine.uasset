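; BP_AreaCine is a trigger area that gives BP_Player a faster, more intense cinematic feel while inside its box.
; Overlap begin and end switch walk speed, assign the BPC_Shake camera shake, and play or reverse a timeline that widens the camera FOV.
; While the player is inside, Tick pulses the vignette on the POST post-process volume with a sine wave and prints the value.
; Exit stops the pulse without resetting the vignette.
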(event OnComponentBeginOverlap(Box)
  (params (OverlappedComponent :type Primitive%20Component%20Object%20Reference) (OtherActor :type Actor%20Object%20Reference) (OtherComp :type Primitive%20Component%20Object%20Reference) (OtherBodyIndex :type Integer) (bFromSweep :type Boolean) (SweepResult :type Hit%20Result%20Structure%20%28by%20ref%29))
  (bind _asbp_player (Utilities|Casting|CastToBP_Player OtherActor))
  (bind _output_get (Variables|Default|SetAs%20BP%20Player _asbp_player))
  (Variables|/Script/Engine.CameraShakeSourceComponent|SetCameraShake (Variables|/Game/Somium2/Blueprints/Player/BP_Player.BP_Player_C|GetCameraShakeSource _output_get) "/Game/Somium2/Blueprints/Player/BPC_Shake.BPC_Shake_C")
  (Variables|/Script/Engine.CharacterMovementComponent|SetMaxWalkSpeed (Variables|/Script/Engine.Character|GetCharacterMovement _output_get) 8e+02)
  (Variables|Default|SetCondition true)
  (bind _lerp (Timeline|Change Play)
    (:Update
      (if (Variables|Default|GetCondition)
        (Camera|SetFieldOfView (Variables|/Game/Somium2/Blueprints/Player/BP_Player.BP_Player_C|GetCamera _output_get) (Math|Float|Lerp 1.1e+02 125.0 _lerp))
        (else
          (Camera|SetFieldOfView (Variables|/Game/Somium2/Blueprints/Player/BP_Player.BP_Player_C|GetCamera (stale OnComponentEndOverlap(Box) _output_get)) (Math|Float|Lerp 1.1e+02 125.0 _lerp)))))))

(event OnComponentEndOverlap(Box)
  (params (OverlappedComponent :type Primitive%20Component%20Object%20Reference) (OtherActor :type Actor%20Object%20Reference) (OtherComp :type Primitive%20Component%20Object%20Reference) (OtherBodyIndex :type Integer))
  (bind _asbp_player (Utilities|Casting|CastToBP_Player OtherActor))
  (bind _output_get (Variables|Default|SetAs%20BP%20Player _asbp_player))
  (Variables|/Script/Engine.CameraShakeSourceComponent|SetCameraShake (Variables|/Game/Somium2/Blueprints/Player/BP_Player.BP_Player_C|GetCameraShakeSource _output_get) "/Game/Somium2/Blueprints/Player/BPC_Shake.BPC_Shake_C")
  (Variables|/Script/Engine.CharacterMovementComponent|SetMaxWalkSpeed (Variables|/Script/Engine.Character|GetCharacterMovement _output_get) 4e+02)
  (Variables|Default|SetCondition false)
  (bind _lerp (Timeline|Change Reverse)
    (:Update
      (if (Variables|Default|GetCondition)
        (Camera|SetFieldOfView (Variables|/Game/Somium2/Blueprints/Player/BP_Player.BP_Player_C|GetCamera (stale OnComponentBeginOverlap(Box) _output_get)) (Math|Float|Lerp 1.1e+02 125.0 _lerp))
        (else
          (Camera|SetFieldOfView (Variables|/Game/Somium2/Blueprints/Player/BP_Player.BP_Player_C|GetCamera _output_get) (Math|Float|Lerp 1.1e+02 125.0 _lerp)))))))

(event EventTick
  (params (DeltaSeconds :type Float%20%28single-precision%29))
  (bind _returnvalue (Utilities|Time|GetTimeSeconds))
  (bind _returnvalue_2 (* _returnvalue 2.0))
  (bind _returnvalue_3 (Math|Trig|Sin(Radians) _returnvalue_2))
  (bind _returnvalue_4 (Math|Float|Absolute(Float) _returnvalue_3))
  (bind _returnvalue_5 (Math|Float|Lerp 0.6 1.0 _returnvalue_4))
  (if (Variables|Default|GetCondition)
    (bind _aspost_process_volume (Utilities|Casting|CastToPostProcessVolume (Variables|Default|GetPOST)))
    (Development|PrintString (Utilities|String|ToString(Float) _returnvalue_5))
    (Utilities|Struct|SetmembersinPostProcessSettings (Variables|/Script/Engine.PostProcessVolume|GetSettings _aspost_process_volume) _returnvalue_5)))

(fn ConstructionScript)