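; Floating widget actor meant to display the ID of a BP_Recepteur or BP_Scanner in WBP_FréquenceAnim and face the player.
; All of that logic is disconnected: BeginPlay, Tick and the construction script do nothing.
; The unwired setup reads the ID from the parent actor, falling back to ActorIndependant, and updates the widget text.
; Unwired look-at fragments rotate it toward the player, gated by Indepandant or ActorIndependant validity.
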(event EventTick
  (params (DeltaSeconds :type Float%20%28single-precision%29))
  ;[1 1 1] Comment
)

(event EventBeginPlay)

(fn ConstructionScript)