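; BP_Recepteur is a receiver that opens a linked locked door and activates its exit panel.
; On BeginPlay it spawns a BP_Drone_Stockage, registers itself as its owner and attaches it to ObjectTarget.
; OpenDoor briefly unlocks LockedDoor to toggle it, re-locks it, then triggers ExitPanel.
; The construction script adds a small sprite above the actor when LockedDoor is invalid or ID is zero, flagging incomplete setup.
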(event Custom|OpenDoor
  (bind _lockeddoor (Variables|LockDoor|GetLockedDoor))
  (Variables|/Game/Somium2/Blueprints/GPE/BP_Door.BP_Door_C|SetIsDoorLocked? _lockeddoor false)
  (Default|Open/CloseDoor _lockeddoor)
  (Variables|/Game/Somium2/Blueprints/GPE/BP_Door.BP_Door_C|SetIsDoorLocked? _lockeddoor true)
  (Default|ActivateEvent (Variables|LockDoor|GetExitPanel)))

(event EventBeginPlay
  ;[1 1 1] EVENT BEGIN
  (bind _returnvalue (Game|SpawnActorfromClass "/Game/Somium2/Blueprints/GPE/Robot_MSE-6/BP_Drone_Stockage.BP_Drone_Stockage_C" (Transformation|GetActorTransform) "Undefined" 0 0))
  (Variables|/Game/Somium2/Blueprints/GPE/Robot_MSE-6/BP_Drone_Stockage.BP_Drone_Stockage_C|SetRecepteurOwner _returnvalue self)
  (Transformation|AttachComponentToComponent _returnvalue (Variables|Default|GetObjectTarget) "None" "SnapToTarget" "SnapToTarget" "SnapToTarget" true))

(fn ConstructionScript
  (Variables|LockDoor|GetLockedDoor
    (:then
      (if (== (Variables|LockDoor|GetID) 0)
        (AddComponent|AddPaperSpriteComponent false (Math|Transform|MakeTransform (Math|Vector|MakeVector 0.0 0.0 1e+02) "0, 0, 0" "0.100000,0.100000,0.100000") :!label _label)))
    (:else
      (goto _label))))