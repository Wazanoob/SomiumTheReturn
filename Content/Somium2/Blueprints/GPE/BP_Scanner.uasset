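; BP_Scanner is a scanner gameplay element whose mesh color shows idle, failure (Echec) and win feedback.
; Tick pulses material slot 1 between Idle and black by sine, recreating the dynamic material instance each frame, unless Anim is set.
; EchecEvent plays a red timeline, then resumes pulsing.
; WinEvent ends frequency animation widgets on its child actor and external screens, then plays a green timeline, leaving the pulse off.
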(event Custom|Echec%20Event
  (bind _staticmesh (Variables|Default|GetStaticMesh))
  ;[1 1 1] Comment
  (bind _returnvalue (Rendering|Material|CreateDynamicMaterialInstance _staticmesh 1 (Rendering|Material|GetMaterial _staticmesh 1) "None" :!class /Script/Engine.PrimitiveComponent))
  (bind _value (Timeline|Change PlayFromStart)
    (:Update
      (Variables|Default|SetAnim true)
      (Rendering|Material|SetVectorParameterValue _returnvalue "Color Multiply" (Math|Color|Lerp(LinearColor) (Variables|Default|GetIdle) "(R=0.572917,G=0.000000,B=0.000000,A=1.000000)" _value) :!class /Script/Engine.MaterialInstanceDynamic))
    (:Finished
      (Variables|Default|SetAnim false))))

(event Custom|Win%20Event
  ;[1 1 1] Comment
  (bind _returnvalue (Rendering|Material|CreateDynamicMaterialInstance (Variables|Default|GetStaticMesh) 1 (Rendering|Material|GetMaterial (Variables|Default|GetStaticMesh) 1) "None" :!class /Script/Engine.PrimitiveComponent))
  (bind _asbp_widget_floating (Utilities|Casting|CastToBP_WidgetFloating (Variables|/Script/Engine.ChildActorComponent|GetChildActor (Variables|Default|GetChildActor))))
  (bind _aswbp_fréquence_anim (Utilities|Casting|CastToWBP_FréquenceAnim (UserInterface|GetWidget (Variables|/Game/Somium2/Blueprints/BP_WidgetFloating.BP_WidgetFloating_C|GetWidget _asbp_widget_floating))))
  (Default|End _aswbp_fréquence_anim)
  (for _array_element (Variables|Default|GetExternalScreen)
    (bind _aswbp_fréquence_anim_2 (Utilities|Casting|CastToWBP_FréquenceAnim (UserInterface|GetWidget (Variables|/Game/Somium2/Blueprints/BP_WidgetFloating.BP_WidgetFloating_C|GetWidget _array_element))))
    (Default|End _aswbp_fréquence_anim_2))
  (bind _value (Timeline|Timeline_0 Play)
    (:Update
      (Variables|Default|SetAnim true)
      (Rendering|Material|SetVectorParameterValue _returnvalue "Color Multiply" (Math|Color|Lerp(LinearColor) (Variables|Default|GetIdle) "(R=0.051195,G=0.848958,B=0.069802,A=1.000000)" _value) :!class /Script/Engine.MaterialInstanceDynamic))
    (:Finished
      (Variables|Default|SetAnim true))))

(event EventTick
  (params (DeltaSeconds :type Float%20%28single-precision%29))
  (bind _staticmesh (Variables|Default|GetStaticMesh))
  (if (not (Variables|Default|GetAnim))
    (bind _returnvalue (Rendering|Material|CreateDynamicMaterialInstance _staticmesh 1 (Rendering|Material|GetMaterial _staticmesh 1) "None" :!class /Script/Engine.PrimitiveComponent))
    (Rendering|Material|SetVectorParameterValue _returnvalue "Color Multiply" (Math|Color|Lerp(LinearColor) :A (Variables|Default|GetIdle) :Alpha (Math|Trig|Sin(Radians) (* (Utilities|Time|GetTimeSeconds) 2.0))) :!class /Script/Engine.MaterialInstanceDynamic)))

(event EventBeginPlay
  (bind _returnvalue (Rendering|Material|CreateDynamicMaterialInstance (Variables|Default|GetStaticMesh) 1 (Rendering|Material|GetMaterial (Variables|Default|GetStaticMesh) 1) "None" :!class /Script/Engine.PrimitiveComponent))
  (Rendering|Material|SetVectorParameterValue _returnvalue "Color Multiply" (Variables|Default|GetIdle) :!class /Script/Engine.MaterialInstanceDynamic))

(fn ConstructionScript)