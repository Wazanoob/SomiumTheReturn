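; BP_RadioactivZone is a radioactive area trigger that changes the player's HUD and audio while they are inside its box.
; Box overlaps with BP_Player start or end the radioactive state on the player's HUD widget.
; A timeline plays on entry and reverses on exit, lerping the pitch multiplier of the player's AudioCurveSource between normal and half.
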(event OnComponentBeginOverlap(Box)
  (params (OverlappedComponent :type Primitive%20Component%20Object%20Reference) (OtherActor :type Actor%20Object%20Reference) (OtherComp :type Primitive%20Component%20Object%20Reference) (OtherBodyIndex :type Integer) (bFromSweep :type Boolean) (SweepResult :type Hit%20Result%20Structure%20%28by%20ref%29))
  (bind _asbp_player (Utilities|Casting|CastToBP_Player OtherActor))
  (Default|RadioActiveAera (Variables|/Game/Somium2/Blueprints/Player/BP_Player.BP_Player_C|GetHud_Widget _asbp_player))
  (Variables|Default|SetAudio%20Curve%20Source (Variables|/Game/Somium2/Blueprints/Player/BP_Player.BP_Player_C|GetAudioCurveSource _asbp_player))
  (bind _newtrack_0 (Timeline|Value Play)
    (:Update
      (Audio|Components|Audio|SetPitchMultiplier (Variables|Default|GetAudio%20Curve%20Source) (Math|Float|Lerp 1.0 0.5 _newtrack_0)))))

(event OnComponentEndOverlap(Box)
  (params (OverlappedComponent :type Primitive%20Component%20Object%20Reference) (OtherActor :type Actor%20Object%20Reference) (OtherComp :type Primitive%20Component%20Object%20Reference) (OtherBodyIndex :type Integer))
  (bind _asbp_player (Utilities|Casting|CastToBP_Player OtherActor))
  (Default|EndRadioactiveArea (Variables|/Game/Somium2/Blueprints/Player/BP_Player.BP_Player_C|GetHud_Widget _asbp_player))
  (Variables|Default|SetAudio%20Curve%20Source (Variables|/Game/Somium2/Blueprints/Player/BP_Player.BP_Player_C|GetAudioCurveSource _asbp_player))
  (bind _newtrack_0 (Timeline|Value Reverse)
    (:Update
      (Audio|Components|Audio|SetPitchMultiplier (Variables|Default|GetAudio%20Curve%20Source) (Math|Float|Lerp 1.0 0.5 _newtrack_0)))))

(event EventBeginPlay)

(event Collision|EventActorBeginOverlap
  (params (OtherActor :type Actor%20Object%20Reference)))

(event EventTick
  (params (DeltaSeconds :type Float%20%28single-precision%29)))

(fn ConstructionScript)