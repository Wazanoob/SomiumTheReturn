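; Sliding four-panel door that opens and closes with sound as things enter or leave its trigger box, unless locked.
; Begin and end overlap both call the same toggle with no actor filter, flipping the closed flag and playing an attenuated sound.
; One timeline drives the side panels along Y and the top and bottom panels along Z in opposing pairs, reversing to close.
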(event OnComponentBeginOverlap(TriggerBox)
  (params (OverlappedComponent :type Primitive%20Component%20Object%20Reference) (OtherActor :type Actor%20Object%20Reference) (OtherComp :type Primitive%20Component%20Object%20Reference) (OtherBodyIndex :type Integer) (bFromSweep :type Boolean) (SweepResult :type Hit%20Result%20Structure%20%28by%20ref%29))
  (CallFunction|Open/CloseDoor))

(event OnComponentEndOverlap(TriggerBox)
  (params (OverlappedComponent :type Primitive%20Component%20Object%20Reference) (OtherActor :type Actor%20Object%20Reference) (OtherComp :type Primitive%20Component%20Object%20Reference) (OtherBodyIndex :type Integer))
  (CallFunction|Open/CloseDoor))

(event Custom|Open/Close%20Door
  (bind _returnvalue (Transformation|GetActorLocation))
  (bind _leftdoor (Variables|Default|GetLeftDoor))
  (bind _rightdoor (Variables|Default|GetRightDoor))
  (bind _downdoor (Variables|Default|GetDownDoor))
  (bind _topdoor (Variables|Default|GetTopDoor))
  (bind _relativelocation (Variables|/Script/Engine.SceneComponent|GetRelativeLocation _topdoor))
  (bind _relativelocation_2 (Variables|/Script/Engine.SceneComponent|GetRelativeLocation _downdoor))
  (bind _relativelocation_3 (Variables|/Script/Engine.SceneComponent|GetRelativeLocation _leftdoor))
  (bind _relativelocation_4 (Variables|/Script/Engine.SceneComponent|GetRelativeLocation _rightdoor))
  (if (not (Variables|Default|GetIsDoorLocked?))
    (if (Variables|Default|GetIsDoorClosed?)
      (Variables|Default|SetIsDoorClosed? false)
      (Audio|PlaySoundatLocation "/Game/FirstPerson/FX/SFX/Sound/Porte/SFX_Door_Open_idea-001_Cue.SFX_Door_Open_idea-001_Cue" _returnvalue "0, 0, 0" 5.0 1.0 0.0 "/Game/FirstPerson/FX/SFX/DistanceAttenuation.DistanceAttenuation" 0 0 0)
      (bind (_direction _middledoors _sidedoors) (Timeline|DoorAnimation Play)
        (:Update
          (Utilities|FlowControl|Sequence
            (:then_0
              (Transformation|SetRelativeLocation _leftdoor (Math|Vector|MakeVector (.x _relativelocation_3) (* _sidedoors -1e+02) (.z _relativelocation_3)) false false)
              (bind _result (Math|Float|NegateFloat (* _sidedoors -1e+02))
                (:%20%20
                  (Transformation|SetRelativeLocation _rightdoor (Math|Vector|MakeVector (.x _relativelocation_4) _result (.z _relativelocation_4)) false false))))
            (:then_1
              (Transformation|SetRelativeLocation _downdoor (Math|Vector|MakeVector (.x _relativelocation_2) (.y _relativelocation_2) (* _middledoors -2e+02)) false false)
              (bind _result_2 (Math|Float|NegateFloat (* _middledoors -2e+02))
                (:%20%20
                  (Transformation|SetRelativeLocation _topdoor (Math|Vector|MakeVector (.x _relativelocation) (.y _relativelocation) _result_2) false false)))))))
      (else
        (Variables|Default|SetIsDoorClosed? true)
        (Audio|PlaySoundatLocation "/Game/FirstPerson/FX/SFX/Sound/Porte/SFX_Door_Close_idea_-002_Cue.SFX_Door_Close_idea_-002_Cue" _returnvalue "0, 0, 0" 5.0 1.0 0.0 "/Game/FirstPerson/FX/SFX/DistanceAttenuation.DistanceAttenuation" 0 0 0)
        (Timeline|DoorAnimation Reverse)))))

(event EventBeginPlay)

(fn ConstructionScript)