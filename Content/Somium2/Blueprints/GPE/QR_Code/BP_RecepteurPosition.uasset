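; Receiver position marker, in the QR Code gameplay elements, whose Type (such as Stairs or Scanner) sets the color of an editor-visible point light that BeginPlay hides in game.
; The construction script also validates setup, adding a small raised Paper sprite when Stairs lacks either door, or Scanner lacks its locked door, scanner or non-zero ID.
; The LockedDoor replication callback is empty.
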(event EventBeginPlay
  (Development|SetHiddeninGame (Variables|Default|GetPointLight) true false))

(fn ConstructionScript
  (bind _pointlight (Variables|Default|GetPointLight))
  (switch Utilities|FlowControl|Switch|SwitchonQR_Type (Variables|Default|GetType)
    (:NewEnumerator0
      (Rendering|Components|Light|SetLightColor _pointlight "(R=0.584011,G=0.601042,B=0.585722,A=1.000000)" true))
    (:NewEnumerator1
      (Rendering|Components|Light|SetLightColor _pointlight "(R=0.000000,G=0.720833,B=0.082534,A=1.000000)" true)
      (Variables|StairsType|GetDoorEntrance
        (:then
          (Variables|StairsType|GetDoorExit
            (:then)
            (:else
              _)))
        (:else
          _))
      (AddComponent|AddPaperSpriteComponent false (Math|Transform|MakeTransform (Math|Vector|MakeVector 0.0 0.0 1e+02) "0, 0, 0" "0.100000,0.100000,0.100000")))
    (:NewEnumerator2
      (Rendering|Components|Light|SetLightColor _pointlight "(R=0.601042,G=0.010087,B=0.000000,A=1.000000)" true)
      (Variables|ScannerType|GetLockedDoor
        (:then
          (if (== (Variables|ScannerType|GetID) 0)
            _
            (else
              (Variables|ScannerType|GetScanner
                (:then)
                (:else
                  _)))))
        (:else
          _))
      (AddComponent|AddPaperSpriteComponent false (Math|Transform|MakeTransform (Math|Vector|MakeVector 0.0 0.0 1e+02) "0, 0, 0" "0.100000,0.100000,0.100000")))))

(fn OnRepLockedDoor)