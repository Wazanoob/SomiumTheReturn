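; BP_GPE_Test is a test gameplay element that the player can pick up, swap with a held object, and highlight.
; Interact drops any valid input actor at this actor's location via SwitchObject, then stores itself in BP_Player's MyActor and hides with collision disabled.
; Scan and outline events drive custom depth stencil values, with separate scan values for the main and Inner meshes and a FlipFlop-toggled outline.
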(event Custom|DesactivateScanDepth
  ;[1 1 1] Scan outline
  (Rendering|SetCustomDepthStencilValue (Variables|Default|GetStaticMesh) 0)
  (Rendering|SetCustomDepthStencilValue (Variables|Default|GetInner) 0))

(event Custom|ActivateScanDepth
  ;[1 1 1] Scan outline
  (Rendering|SetCustomDepthStencilValue (Variables|Default|GetStaticMesh) 2)
  (Rendering|SetCustomDepthStencilValue (Variables|Default|GetInner) 3))

(event EventEnable/DisableOutline
  (bind _staticmesh (Variables|Default|GetStaticMesh))
  (Utilities|FlowControl|FlipFlop
    (:A
      (Rendering|SetCustomDepthStencilValue _staticmesh 1))
    (:B
      (Rendering|SetCustomDepthStencilValue _staticmesh 0))))

(event EventInteract
  (params (InputActor :type Actor%20Object%20Reference) (InputPosition :type Vector :default "0, 0, 0"))
  ;[0 0.3913 1] Interact
  (Utilities|IsValid InputActor
    (:Is%20Valid
      (CallFunction|SwitchObject InputActor))
    (:Is%20Not%20Valid
      _))
  (bind _asbp_player (Utilities|Casting|CastToBP_Player (Game|Player|GetPlayerPawn 0)))
  (Variables|/Game/Somium2/Blueprints/Player/BP_Player.BP_Player_C|SetMyActor _asbp_player self)
  (Rendering|SetActorHiddenInGame true)
  (Collision|SetActorEnableCollision false))

(fn ConstructionScript)

(fn SwitchObject
  (params (ActorToSwitch :type Actor%20Object%20Reference))
  (Transformation|DetachFromActor ActorToSwitch "KeepRelative" "KeepRelative" "KeepRelative")
  (Transformation|SetActorLocation ActorToSwitch (Transformation|GetActorLocation) false true)
  (Rendering|SetActorHiddenInGame ActorToSwitch false)
  (Collision|SetActorEnableCollision ActorToSwitch true))