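; Storage drone Blueprint with a tray that holds one emitter object, exchanged with the player through Interact.
; An incoming object snaps to the StockageBox socket, while SwitchObject hands any held object back to the player hidden, swapping or emptying the tray.
; After a valid deposit, a matching ID opens the RecepteurOwner's door and a drop sound plays.
; A FlipFlop toggles the box's custom-depth stencil for outlining.
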(event EventEnable/DisableOutline
  (bind _stockagebox (Variables|Default|GetStockageBox))
  ;[0 0.3913 1] Enable/disable outline
  (Utilities|FlowControl|FlipFlop
    (:A
      (Rendering|SetCustomDepthStencilValue _stockagebox 1))
    (:B
      (Rendering|SetCustomDepthStencilValue _stockagebox 0))))

(event EventInteract
  (params (InputActor :type Actor%20Object%20Reference) (InputPosition :type Vector :default "0, 0, 0"))
  ;[0.5898 0 0.601] Interaction With Tray
  (Utilities|IsValid InputActor
    (:Is%20Valid
      (Utilities|FlowControl|Sequence
        (:then_0
          (if (not (Variables|Default|GetIsCarryingObject))
            (Transformation|AttachComponentToComponent InputActor (Variables|Default|GetStockageBox) "ObjectTarget" "SnapToTarget" "SnapToTarget" "KeepRelative" true)
            (Rendering|SetActorHiddenInGame InputActor false)
            (Collision|SetActorEnableCollision InputActor false)
            (bind _asbp_emetteur_object (Utilities|Casting|CastToBP_EmetteurObject InputActor))
            (Variables|Default|SetMyCarryingObject _asbp_emetteur_object)
            (bind _asbp_player (Utilities|Casting|CastToBP_Player (Game|Player|GetPlayerPawn 0)))
            (Variables|/Game/Somium2/Blueprints/Player/BP_Player.BP_Player_C|SetMyActor _asbp_player 0)
            (Variables|Default|SetIsCarryingObject true)
            (else
              (CallFunction|SwitchObject InputActor))))
        (:then_1
          (bind _recepteurowner (Variables|Default|GetRecepteurOwner)
            (:then
              (if (== (Variables|/Game/Somium2/Blueprints/GPE/BP_EmetteurObject.BP_EmetteurObject_C|GetID (Variables|Default|GetMyCarryingObject)) (Variables|/Game/Somium2/Blueprints/GPE/BP_Recepteur.BP_Recepteur_C|GetID _recepteurowner))
                (Default|OpenDoor (Variables|Default|GetRecepteurOwner))))
            (:else)))
        (:then_2
          (Audio|PlaySoundatLocation "/Game/Somium2/Sounds/MS_DropItem.MS_DropItem" (Transformation|GetActorLocation) "0, 0, 0" 1.0 1.0 0.0 "/Game/FirstPerson/FX/SFX/DistanceAttenuation.DistanceAttenuation" 0 0 0))))
    (:Is%20Not%20Valid
      (CallFunction|SwitchObject))))

(fn ConstructionScript)

(fn SwitchObject
  (params (ActorToSwitch :type Actor%20Object%20Reference))
  (Utilities|IsValid ActorToSwitch
    (:Is%20Valid
      (Transformation|AttachComponentToComponent ActorToSwitch (Variables|Default|GetStockageBox) "ObjectTarget" "SnapToTarget" "SnapToTarget" "KeepRelative" true)
      (Rendering|SetActorHiddenInGame ActorToSwitch false)
      (Rendering|SetActorHiddenInGame (Variables|Default|GetMyCarryingObject) true)
      (bind _asbp_player (Utilities|Casting|CastToBP_Player (Game|Player|GetPlayerPawn 0)))
      (Variables|/Game/Somium2/Blueprints/Player/BP_Player.BP_Player_C|SetMyActor _asbp_player (Variables|Default|GetMyCarryingObject))
      (bind _asbp_emetteur_object (Utilities|Casting|CastToBP_EmetteurObject ActorToSwitch))
      (Variables|Default|SetMyCarryingObject _asbp_emetteur_object))
    (:Is%20Not%20Valid
      (bind _mycarryingobject (Variables|Default|GetMyCarryingObject)
        (:then
          (Rendering|SetActorHiddenInGame _mycarryingobject true)
          (bind _asbp_player_2 (Utilities|Casting|CastToBP_Player (Game|Player|GetPlayerPawn 0)))
          (Variables|/Game/Somium2/Blueprints/Player/BP_Player.BP_Player_C|SetMyActor _asbp_player_2 (Variables|Default|GetMyCarryingObject))
          (Variables|Default|SetMyCarryingObject 0)
          (Variables|Default|SetIsCarryingObject false))
        (:else)))))