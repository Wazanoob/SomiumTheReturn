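; MSE-6 drone robot that travels to an interacted position, carrying a spawned storage actor attached to its mesh.
; It follows a synchronous navmesh path point by point, rotating in place toward each before AI MoveTo.
; A special QR appends a stop: stairs teleport it between robot doors, scanners open a locked door if the carried object's ID matches.
; A flip-flop toggles its custom-depth stencil outline.
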(event Custom|RobotMoveTo
  (params (TargetPosition :type Vector))
  ;[0 0.3913 1] Move to
  (Variables|Pathfinding|SetCurrentIndexPosition 0)
  (bind _returnvalue (Class|NavigationSystemV1|FindPathtoLocationSynchronously (Transformation|GetActorLocation) TargetPosition 0 0))
  (Variables|Pathfinding|SetPath%20Points (Variables|/Script/NavigationSystem.NavigationPath|GetPathPoints _returnvalue))
  (CallFunction|GotoNextPosition)
  (Variables|Default|SetShouldMove? true)
  (Variables|Default|SetCanInteract false))

(event Custom|ResetStopMove
  ;[0.601 0.3388 0] EVENT TICK
  ;;[0 0.3913 1] Robot movement
  (Utilities|FlowControl|DoOnce false) ; enters at Reset
)

(event EventEnable/DisableOutline
  (bind _mesh (Variables|Character|GetMesh))
  ;[0 0.3913 1] Enable/disable outline
  (Utilities|FlowControl|FlipFlop
    (:A
      (Rendering|SetCustomDepthStencilValue _mesh 1))
    (:B
      (Rendering|SetCustomDepthStencilValue _mesh 0))))

(event EventInteract
  (params (InputActor :type Actor%20Object%20Reference) (InputPosition :type Vector :default "0, 0, 0"))
  ;[0.5898 0 0.601] Interact With Robot
  (if (Variables|Default|GetCanInteract)
    (Utilities|FlowControl|Sequence
      (:then_0
        (CallFunction|RobotMoveto InputPosition))
      (:then_1
        (bind _specialqr (Variables|Default|GetSpecialQR)
          (:then
            (switch Utilities|FlowControl|Switch|SwitchonQR_Type (Variables|/Game/Somium2/Blueprints/GPE/QR_Code/BP_RecepteurPosition.BP_RecepteurPosition_C|GetType _specialqr)
              (:NewEnumerator1
                (Utilities|Array|Add (Variables|Pathfinding|GetPath%20Points) (Transformation|GetActorLocation (Variables|/Game/Somium2/Blueprints/GPE/QR_Code/BP_RecepteurPosition.BP_RecepteurPosition_C|GetDoorEntrance _specialqr))))
              (:NewEnumerator2
                (Utilities|Array|Add (Variables|Pathfinding|GetPath%20Points) (Transformation|GetActorLocation (Variables|/Game/Somium2/Blueprints/GPE/QR_Code/BP_RecepteurPosition.BP_RecepteurPosition_C|GetScanner _specialqr))))))
          (:else))))))

(event EventBeginPlay
  ;[0 1 0.1182] EVENT BEGIN
  (bind _returnvalue (Game|SpawnActorfromClass "/Game/Somium2/Blueprints/GPE/Robot_MSE-6/BP_Drone_Stockage.BP_Drone_Stockage_C" (Transformation|GetActorTransform) "Undefined" 0 0))
  (bind _output_get (Variables|Default|SetMyStockage _returnvalue))
  (Transformation|AttachComponentToComponent _output_get (Variables|Character|GetMesh) "None" "SnapToTarget" "SnapToTarget" "SnapToTarget" true))

(event EventTick
  (params (DeltaSeconds :type Float%20%28single-precision%29))
  (bind _returnvalue (Transformation|GetActorLocation))
  (bind _nextposition (Variables|Pathfinding|GetNextPosition))
  ;[0.601 0.3388 0] EVENT TICK
  (Utilities|FlowControl|Sequence
    (:then_0
      ;;[0 0.3913 1] Robot movement
      (if (Variables|Default|GetShouldMove?)
        (Utilities|FlowControl|Sequence
          (:then_0
            (if (Variables|Default|GetShouldRotate?)
              (CallFunction|RotateinPlace (Variables|Pathfinding|GetNextPosition) DeltaSeconds)
              (else
                (Utilities|FlowControl|DoOnce false :!label _label
                  (:Completed
                    (AI|AIMoveTo self (Variables|Pathfinding|GetNextPosition) 0 5.0 false))))))
          (:then_1
            (if (and (<= (Math|Float|Absolute(Float) (- (.x _returnvalue) (.x _nextposition))) 5.0) (<= (Math|Float|Absolute(Float) (- (.y _returnvalue) (.y _nextposition))) 5.0))
              (CallFunction|GotoNextPosition)
              (goto _label Reset))))
        (else
          (Utilities|FlowControl|DoOnce false
            (:Completed
              (Class|NavMovementComponent|StopActiveMovement (Variables|Character|GetCharacterMovement))
              (CallFunction|GotoExit))))))))

(fn ConstructionScript)

(fn RotateinPlace
  (params (TargetDestination :type Vector) (DeltaSeconds :type Float%20%28double-precision%29))
  (bind _capsulecomponent (Variables|Collision|GetCapsuleComponent))
  (Transformation|SetWorldRotation (Variables|Collision|GetCapsuleComponent) (Math|Interpolation|RInterpTo (Transformation|GetWorldRotation _capsulecomponent) (Math|Rotator|FindLookatRotation (Transformation|GetWorldLocation _capsulecomponent) TargetDestination) DeltaSeconds 2.0) false false)
  (CallFunction|CheckforRotation))

(fn CheckforRotation
  (bind _capsulecomponent (Variables|Collision|GetCapsuleComponent))
  (if (Utilities|Operators|EqualEqual (Transformation|GetWorldRotation _capsulecomponent) (Math|Rotator|FindLookatRotation (Transformation|GetWorldLocation _capsulecomponent) (Variables|Pathfinding|GetNextPosition)) 5.0)
    (Variables|Default|SetShouldRotate? false)
    (else
      (Variables|Default|SetShouldRotate? true))))

(fn GotoNextPosition
  (bind _returnvalue (Transformation|GetActorRotation))
  (bind _path_points (Variables|Pathfinding|GetPath%20Points))
  (bind _currentindexposition (Variables|Pathfinding|GetCurrentIndexPosition))
  (bind _output (Utilities|Array|Get(acopy) _path_points _currentindexposition))
  (CallFunction|ResetStopMove)
  (Math|Integer|IncrementInt (Variables|Pathfinding|GetCurrentIndexPosition)
    (:%20%20
      (if (> (Variables|Pathfinding|GetCurrentIndexPosition) (Utilities|Array|LastIndex (Variables|Pathfinding|GetPath%20Points)))
        (Variables|Default|SetShouldMove? false)
        (bind _specialqr (Variables|Default|GetSpecialQR)
          (:then
            (switch Utilities|FlowControl|Switch|SwitchonQR_Type (Variables|/Game/Somium2/Blueprints/GPE/QR_Code/BP_RecepteurPosition.BP_RecepteurPosition_C|GetType _specialqr)
              (:NewEnumerator1
                ;[0 0.3913 1] Teleport to Exit Robot Door
                (Utilities|FlowControl|DoOnce false
                  (:Completed
                    (Transformation|SetActorLocation (Transformation|GetActorLocation (Variables|/Game/Somium2/Blueprints/GPE/QR_Code/BP_RecepteurPosition.BP_RecepteurPosition_C|GetDoorExit _specialqr)) false true)
                    (Transformation|SetActorRotation (Math|Rotator|MakeRotator (.roll _returnvalue) (.pitch _returnvalue) (+ (.yaw _returnvalue) 1.8e+02)) true))))
              (:NewEnumerator2
                ;[0 0.3913 1] Scan Robot carrying object ID to unlock door
                (Utilities|FlowControl|DoOnce false
                  (:Completed
                    (bind _mycarryingobject (Variables|/Game/Somium2/Blueprints/GPE/Robot_MSE-6/BP_Drone_Stockage.BP_Drone_Stockage_C|GetMyCarryingObject (Variables|Default|GetMyStockage))
                      (:then
                        (if (== (Variables|/Game/Somium2/Blueprints/GPE/BP_EmetteurObject.BP_EmetteurObject_C|GetID _mycarryingobject) (Variables|/Game/Somium2/Blueprints/GPE/QR_Code/BP_RecepteurPosition.BP_RecepteurPosition_C|GetID _specialqr))
                          (Variables|/Game/Somium2/Blueprints/GPE/BP_Door.BP_Door_C|SetIsDoorLocked? (Variables|/Game/Somium2/Blueprints/GPE/QR_Code/BP_RecepteurPosition.BP_RecepteurPosition_C|GetLockedDoor _specialqr) false)
                          (Default|Open/CloseDoor (Variables|/Game/Somium2/Blueprints/GPE/QR_Code/BP_RecepteurPosition.BP_RecepteurPosition_C|GetLockedDoor _specialqr))
                          (Variables|/Game/Somium2/Blueprints/GPE/BP_Door.BP_Door_C|SetIsDoorLocked? (Variables|/Game/Somium2/Blueprints/GPE/QR_Code/BP_RecepteurPosition.BP_RecepteurPosition_C|GetLockedDoor _specialqr) true)
                          (CallFunction|RobotMoveto (Transformation|GetActorLocation _specialqr))
                          (else
                            (CallFunction|RobotMoveto (Transformation|GetActorLocation _specialqr) :!label _label))))
                      (:else
                        (goto _label))))))))
          (:else
            (Variables|Default|SetCanInteract true)))
        (else
          (Variables|Pathfinding|SetNextPosition (Math|Vector|MakeVector (.x _output) (.y _output) (.z (Transformation|GetActorLocation))))
          (CallFunction|CheckforRotation))))))

(fn GotoExit
  (Variables|Default|GetSpecialQR
    (:then
      (if (Utilities|Enum|Equal(Enum) (Variables|/Game/Somium2/Blueprints/GPE/QR_Code/BP_RecepteurPosition.BP_RecepteurPosition_C|GetType (Variables|Default|GetSpecialQR)) "NewEnumerator1")
        (CallFunction|RobotMoveto (+ (* (Transformation|GetActorForwardVector (Variables|/Game/Somium2/Blueprints/GPE/QR_Code/BP_RecepteurPosition.BP_RecepteurPosition_C|GetDoorExit (Variables|Default|GetSpecialQR))) 1e+02) (Transformation|GetActorLocation (Variables|/Game/Somium2/Blueprints/GPE/QR_Code/BP_RecepteurPosition.BP_RecepteurPosition_C|GetDoorExit (Variables|Default|GetSpecialQR)))))
        (Variables|Default|SetSpecialQR 0)))
    (:else)))