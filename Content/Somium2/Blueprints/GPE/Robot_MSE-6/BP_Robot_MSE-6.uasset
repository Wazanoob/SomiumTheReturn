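; MSE-6 robot pawn that, on interaction, travels to the supplied position and can toggle a stencil-based outline.
; It computes a navigation path synchronously, then Tick steps through the points, turning the capsule toward each before issuing AIMoveTo.
; A loose XY distance check advances to the next point and stops movement after the last.
; Object carrying and swapping with BP_Player via a mesh socket exists but is disconnected.
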(event Custom|RobotMoveTo
  (params (TargetPosition :type Vector))
  ;[0 0.3913 1] Move to
  (Variables|Pathfinding|SetCurrentIndexPosition 0)
  (bind _returnvalue (Class|NavigationSystemV1|FindPathtoLocationSynchronously (Transformation|GetActorLocation) TargetPosition 0 0))
  (Variables|Pathfinding|SetPath%20Points (Variables|/Script/NavigationSystem.NavigationPath|GetPathPoints _returnvalue))
  (CallFunction|GotoNextPosition)
  (Variables|Default|SetShouldMove? true))

(event EventEnable/DisableOutline
  (bind _mesh (Variables|Character|GetMesh))
  ;[0 0.3913 1] Enable/disable outline
  (Utilities|FlowControl|FlipFlop
    (:A
      (Rendering|SetCustomDepthStencilValue _mesh 1))
    (:B
      (Rendering|SetCustomDepthStencilValue _mesh 0))))

(event EventInteract
  (params (InputActor :type Actor%20Object%20Reference) (InputPosition :type Vector :default "0, 0, 0"))
  ;[0.5898 0 0.601] Interaction With Tray
  ;[0.5898 0 0.601] Interact With Robot
  (CallFunction|RobotMoveto InputPosition))

(event EventTick
  (params (DeltaSeconds :type Float%20%28single-precision%29))
  (bind _returnvalue (Transformation|GetActorLocation))
  (bind _nextposition (Variables|Pathfinding|GetNextPosition))
  ;[0.601 0.3388 0] EVENT TICK
  (Utilities|FlowControl|Sequence
    (:then_0
      ;;[0 0.3913 1] Robot movement
      (if (Variables|Default|GetShouldMove?)
        (Utilities|FlowControl|Sequence
          (:then_0
            (if (Variables|Default|GetShouldRotate?)
              (CallFunction|RotateinPlace (Variables|Pathfinding|GetNextPosition) DeltaSeconds)
              (else
                (Utilities|FlowControl|DoOnce false :!label _label
                  (:Completed
                    (AI|AIMoveTo self (Variables|Pathfinding|GetNextPosition) 0 5.0 false))))))
          (:then_1
            (if (and (<= (Math|Float|Absolute(Float) (- (.x _returnvalue) (.x _nextposition))) 5.0) (<= (Math|Float|Absolute(Float) (- (.y _returnvalue) (.y _nextposition))) 5.0))
              (CallFunction|GotoNextPosition)
              (goto _label Reset))))))))

(fn ConstructionScript)

(fn RotateinPlace
  (params (TargetDestination :type Vector) (DeltaSeconds :type Float%20%28double-precision%29))
  (bind _capsulecomponent (Variables|Collision|GetCapsuleComponent))
  (Transformation|SetWorldRotation (Variables|Collision|GetCapsuleComponent) (Math|Interpolation|RInterpTo (Transformation|GetWorldRotation _capsulecomponent) (Math|Rotator|FindLookatRotation (Transformation|GetWorldLocation _capsulecomponent) TargetDestination) DeltaSeconds 2.0) false false)
  (CallFunction|CheckforRotation))

(fn CheckforRotation
  (bind _capsulecomponent (Variables|Collision|GetCapsuleComponent))
  (if (Utilities|Operators|EqualEqual (Transformation|GetWorldRotation _capsulecomponent) (Math|Rotator|FindLookatRotation (Transformation|GetWorldLocation _capsulecomponent) (Variables|Pathfinding|GetNextPosition)) 5.0)
    (Variables|Default|SetShouldRotate? false)
    (Development|PrintString "Done")
    (else
      (Variables|Default|SetShouldRotate? true))))

(fn GotoNextPosition
  (bind _path_points (Variables|Pathfinding|GetPath%20Points))
  (bind _currentindexposition (Variables|Pathfinding|GetCurrentIndexPosition))
  (bind _output (Utilities|Array|Get(acopy) _path_points _currentindexposition))
  (Math|Integer|IncrementInt (Variables|Pathfinding|GetCurrentIndexPosition)
    (:%20%20
      (if (> (Variables|Pathfinding|GetCurrentIndexPosition) (Utilities|Array|LastIndex (Variables|Pathfinding|GetPath%20Points)))
        (Variables|Default|SetShouldMove? false)
        (else
          (Variables|Pathfinding|SetNextPosition (Math|Vector|MakeVector (.x _output) (.y _output) (.z (Transformation|GetActorLocation))))
          (CallFunction|CheckforRotation))))))

(fn SwitchObject
  (params (ActorToSwitch :type Actor%20Object%20Reference))
  (Transformation|AttachComponentToComponent ActorToSwitch (Variables|Character|GetMesh) "ObjectTarget" "SnapToTarget" "SnapToTarget" "KeepRelative" true)
  (Rendering|SetActorHiddenInGame ActorToSwitch false)
  (Rendering|SetActorHiddenInGame (Variables|Default|GetMyCarryingObject) true)
  (bind _asbp_player (Utilities|Casting|CastToBP_Player (Game|Player|GetPlayerPawn 0)))
  (Variables|/Game/Somium2/Blueprints/Player/BP_Player.BP_Player_C|SetMyActor _asbp_player (Variables|Default|GetMyCarryingObject))
  (Variables|Default|SetMyCarryingObject ActorToSwitch))