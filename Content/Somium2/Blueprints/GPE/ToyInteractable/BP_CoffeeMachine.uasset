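; Interactable coffee machine prop that fills a mug and empties it again when used.
; Interact locks reuse, turns the light red and, after a delay, plays pour effects while a timeline raises the Sphere as liquid.
; A sip sound and a reversed second timeline lower and hide it, then the light turns green and interaction unlocks.
; A FlipFlop toggles the outline through custom depth stencil.
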(event EventEnable/DisableOutline
  (bind _coffeemachin (Variables|Default|GetCoffeeMachin))
  ;[1 1 1] Outline
  (Utilities|FlowControl|FlipFlop
    (:A
      (Rendering|SetCustomDepthStencilValue _coffeemachin 4))
    (:B
      (Rendering|SetCustomDepthStencilValue _coffeemachin 0))))

(event EventInteract
  (params (InputActor :type Actor%20Object%20Reference) (InputPosition :type Vector :default "0, 0, 0"))
  (bind _sphere (Variables|Default|GetSphere))
  (bind _pointlight (Variables|Default|GetPointLight))
  (if (Variables|Default|GetCanInteract)
    (Variables|Default|SetCanInteract false)
    (Audio|PlaySoundatLocation "/Game/Somium2/Sounds/SFX_ActivateMachine.SFX_ActivateMachine" (+ (Transformation|GetActorLocation) "0,0.000000,100.000000") "0, 0, 0" 1.0 1.0 0.0 "/Game/FirstPerson/FX/SFX/DistanceAttenuation.DistanceAttenuation" 0 0 0)
    (Rendering|Components|Light|SetLightColor _pointlight "(R=0.666667,G=0.097222,B=0.097222,A=1.000000)" true)
    (Utilities|FlowControl|Delay 2.4)
    (Audio|PlaySoundatLocation "/Game/Somium2/Sounds/SFX_Coffee.SFX_Coffee" (Transformation|GetWorldLocation (Variables|Default|GetMug)) "0, 0, 0" 1.0 1.0 0.0 "/Game/FirstPerson/FX/SFX/DistanceAttenuation.DistanceAttenuation" 0 0 0)
    (Development|SetHiddeninGame (Variables|Default|GetSphere) false false)
    (bind _returnvalue (Niagara|SpawnSystemAttached "/Game/Somium2/ART/VFX/SFX_Fluid.SFX_Fluid" (Variables|Default|GetCoffeTarget) "None" "0, 0, 0" "0, 0, 0" "KeepRelativeOffset" true))
    (bind _position (Timeline|Timeline_0 PlayFromStart)
      (:Update
        (Transformation|SetRelativeLocation (Variables|Default|GetSphere) (Math|Vector|MakeVector 0.0 0.0 (* _position 7.0)) false false))
      (:Finished
        (Components|DestroyComponent _returnvalue)
        (Audio|PlaySoundatLocation "/Game/Somium2/Sounds/SFX_CoffeeSip.SFX_CoffeeSip" (Transformation|GetWorldLocation (Variables|Default|GetMug)) "0, 0, 0" 1.0 1.0 0.0 "/Game/FirstPerson/FX/SFX/DistanceAttenuation.DistanceAttenuation" 0 0 0)
        (bind _position_2 (Timeline|Timeline_1 ReverseFromEnd)
          (:Update
            (Transformation|SetRelativeLocation _sphere (Math|Vector|MakeVector 0.0 0.0 (* _position_2 7.0)) false false))
          (:Finished
            (Development|SetHiddeninGame _sphere true false)
            (Variables|Default|SetCanInteract true)
            (Rendering|Components|Light|SetLightColor _pointlight "(R=0.170355,G=0.453125,B=0.186495,A=1.000000)" true)))))))

(fn ConstructionScript)