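; BP_ComputerFlappyBird is an interactable computer prop whose screen switches on and off; despite its name, it contains no game logic.
; BeginPlay creates dynamic material instances for both screen material slots.
; Each interaction flip-flops one material's emissive multiplier between bright and dim, while a timeline plays or reverses to animate the other's.
; An outline event toggles the screen's custom depth stencil value through its own flip-flop.
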(event EventEnable/DisableOutline
  (bind _screen (Variables|Default|GetScreen))
  ;[1 1 1] Outline
  (Utilities|FlowControl|FlipFlop
    (:A
      (Rendering|SetCustomDepthStencilValue _screen 4))
    (:B
      (Rendering|SetCustomDepthStencilValue _screen 0))))

(event EventInteract
  (params (InputActor :type Actor%20Object%20Reference) (InputPosition :type Vector :default "0, 0, 0"))
  (bind _dynamicmaterial (Variables|Default|GetDynamicMaterial))
  (Utilities|FlowControl|FlipFlop
    (:A
      (Rendering|Material|SetScalarParameterValue _dynamicmaterial "Emisive Multiplier" 5.0 :!class /Script/Engine.MaterialInstanceDynamic)
      (bind _emissive (Timeline|Timeline_0 Play)
        (:Update
          (Rendering|Material|SetScalarParameterValue (Variables|Default|GetDynamicMaterial2) "Emisive Multiplier" _emissive :!class /Script/Engine.MaterialInstanceDynamic))))
    (:B
      (Rendering|Material|SetScalarParameterValue _dynamicmaterial "Emisive Multiplier" 0.05 :!class /Script/Engine.MaterialInstanceDynamic)
      (Timeline|Timeline_0 Reverse))))

(event EventBeginPlay
  (bind _returnvalue (Rendering|Material|CreateDynamicMaterialInstance (Variables|Default|GetScreen) 1 "/Game/Somium2/ART/Materials/Props/M_ScreenPC1.M_ScreenPC1" "None" :!class /Script/Engine.PrimitiveComponent))
  (Variables|Default|SetDynamicMaterial _returnvalue)
  (bind _returnvalue_2 (Rendering|Material|CreateDynamicMaterialInstance (Variables|Default|GetScreen) 0 "/Game/Somium2/ART/Materials/Props/M_ScreenPC3.M_ScreenPC3" "None" :!class /Script/Engine.PrimitiveComponent))
  (Variables|Default|SetDynamicMaterial2 _returnvalue_2))

(fn ConstructionScript)