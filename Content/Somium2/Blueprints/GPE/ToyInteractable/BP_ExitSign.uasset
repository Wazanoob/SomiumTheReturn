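; BP_ExitSign is an exit sign toy interactable that swaps color whenever a nearby actor turns its back on it.
; A sphere overlap tracks the nearby actor without filtering for the player.
; Each Tick, a dot product of that actor's forward vector and direction to the sign detects facing away.
; A DoOnce, reset upon facing it again, drives a FlipFlop alternating blue and green materials.
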(event OnComponentBeginOverlap(Sphere)
  (params (OverlappedComponent :type Primitive%20Component%20Object%20Reference) (OtherActor :type Actor%20Object%20Reference) (OtherComp :type Primitive%20Component%20Object%20Reference) (OtherBodyIndex :type Integer) (bFromSweep :type Boolean) (SweepResult :type Hit%20Result%20Structure%20%28by%20ref%29))
  (Variables|Default|SetIsPlayerNearby true)
  (Variables|Default|SetOther%20Actor OtherActor))

(event OnComponentEndOverlap(Sphere)
  (params (OverlappedComponent :type Primitive%20Component%20Object%20Reference) (OtherActor :type Actor%20Object%20Reference) (OtherComp :type Primitive%20Component%20Object%20Reference) (OtherBodyIndex :type Integer))
  (Variables|Default|SetIsPlayerNearby false)
  (Variables|Default|SetOther%20Actor 0))

(event EventTick
  (params (DeltaSeconds :type Float%20%28single-precision%29))
  (bind _other_actor (Variables|Default|GetOther%20Actor))
  (bind _sign (Variables|Default|GetSign))
  (if (Variables|Default|GetIsPlayerNearby)
    (if (<= (Math|Vector|DotProduct (Transformation|GetActorForwardVector _other_actor) (Math|Vector|GetUnitDirection(Vector) (Transformation|GetActorLocation _other_actor) (Transformation|GetActorLocation self))) 0.0)
      (Utilities|FlowControl|DoOnce false :!label _label
        (:Completed
          (Utilities|FlowControl|FlipFlop
            (:A
              (Rendering|Material|SetMaterial _sign 0 "/Game/FirstPerson/ART/Materials/Couleurs/M_Blue.M_Blue"))
            (:B
              (Rendering|Material|SetMaterial _sign 0 "/Game/FirstPerson/ART/Materials/Couleurs/M_Green.M_Green")))))
      (else
        (goto _label Reset)))))

(fn ConstructionScript)