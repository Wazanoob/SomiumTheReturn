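; Interactable toy radio that cycles through on, switch track and off on successive interactions.
; Interact uses two flags to drive an AudioComponent, playing a switch sound for 1.5 seconds before setting the music again.
; Turning on shows music-note VFX, which Tick clears through a resettable DoOnce when off.
; A FlipFlop toggles the mesh's custom depth stencil for the outline.
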(event EventEnable/DisableOutline
  (bind _ph_radio_main (Variables|Default|GetPH_RADIO_MAIN))
  ;[1 1 1] Outline
  (Utilities|FlowControl|FlipFlop
    (:A
      (Rendering|SetCustomDepthStencilValue _ph_radio_main 4))
    (:B
      (Rendering|SetCustomDepthStencilValue _ph_radio_main 0))))

(event EventTick
  (params (DeltaSeconds :type Float%20%28single-precision%29))
  (if (Variables|Default|GetIsEnabled?)
    (goto _label Reset)
    (else
      (Utilities|FlowControl|DoOnce false :!label _label
        (:Completed
          (Class|NiagaraComponent|SetAsset (Variables|Default|GetSFX_MusicNotes) 0 true))))))

(event EventInteract
  (params (InputActor :type Actor%20Object%20Reference) (InputPosition :type Vector :default "0, 0, 0"))
  (bind _audiocomponent (Variables|Default|GetAudioComponent))
  (bind _audiocomponent_2 (Variables|Default|GetAudioComponent))
  ;[0 0.3913 1] Interaction, turn On // Next music // Turn off
  (if (Variables|Default|GetIsEnabled?)
    (if (Variables|Default|GetIsSecondInteract)
      (Variables|Default|SetIsEnabled? false)
      (Variables|Default|SetIsSecondInteract false)
      (Audio|Components|Audio|Stop (Variables|Default|GetAudioComponent))
      (else
        (Variables|Default|SetIsSecondInteract true)
        (Audio|Components|Audio|SetSound _audiocomponent_2 "/Game/Somium2/Sounds/MS_SwitchRadio.MS_SwitchRadio")
        (Utilities|FlowControl|Delay 1.5)
        (Audio|Components|Audio|SetSound _audiocomponent_2 "/Game/Somium2/Sounds/Music/MS_Music.MS_Music")))
    (else
      (Variables|Default|SetIsEnabled? true)
      (Audio|Components|Audio|SetSound _audiocomponent "/Game/Somium2/Sounds/Music/MS_Music.MS_Music")
      (Audio|Components|Audio|Play _audiocomponent 0.0)
      (Class|NiagaraComponent|SetAsset (Variables|Default|GetSFX_MusicNotes) "/Game/Somium2/ART/VFX/SFX_MusicNotes.SFX_MusicNotes" true))))

(fn ConstructionScript)